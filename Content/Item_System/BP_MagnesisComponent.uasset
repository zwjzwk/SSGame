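; Player component for a Magnesis rune that grabs, moves, rotates and attaches BP_Items and scene interactives.
; Rune camera-traces a target into the player's PhysicsHandle or releases it; Tick applies push/pull and camera-relative rotation.
; Release attaches items by nearest attach points, previewed with a debug line found by alternating closest-point-on-collision queries.
; Material swaps highlight grabbable and held objects; a separate Adsorption event snap-combines items.
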(event Custom|Rune
  (bind _player (CallFunction|GetPlayer))
  (bind _componentpickuplocation (Variables|/Game/ThirdPersonCPP/Blueprints/BP_Player.BP_Player_C|GetComponentPickupLocation _player))
  (bind _returnvalue (Transformation|GetWorldRotation _componentpickuplocation))
  (Utilities|IsValid (Variables|Default|GetPhysicsObject)
    (:Is%20Valid
      (Physics|Components|PhysicsHandle|ReleaseComponent (Variables|/Game/ThirdPersonCPP/Blueprints/BP_Player.BP_Player_C|GetPhysicsHandle (CallFunction|GetPlayer)))
      (Variables|Default|SetIsGrabbing false)
      (CallFunction|Attach)
      (Utilities|IsValid (Variables|Default|GetPhysicsObject)
        (:Is%20Valid
          (bind _asbp_item (Utilities|Casting|CastToBP_Item (Components|GetOwner (Variables|Default|GetPhysicsObject)))
            (:then
              (Default|SetMaterialOrigin _asbp_item))
            (:CastFailed
              (bind _asbp_scene_interactive (Utilities|Casting|CastToBP_SceneInteractive (Components|GetOwner (Variables|Default|GetPhysicsObject))))
              (Default|SetMaterialOrigin _asbp_scene_interactive))))
        (:Is%20Not%20Valid
          _))
      (Utilities|FlowControl|Delay 0.4)
      (Variables|Default|SetPhysicsObject 0)
      (Variables|Default|SetMagForce 0.0)
      (Variables|Default|SetMinDistance 5e+02)
      (Variables|Default|SetPointMinDistance (Variables|Default|GetInitialPointMinDistance))
      (Variables|Default|SetPointSelf 0)
      (Variables|Default|SetPointAnother 0)
      (Variables|Default|SetMinDIstanceObject 0))
    (:Is%20Not%20Valid
      (CallFunction|ActiveMagnesisRune)
      (Utilities|IsValid (Variables|Default|GetPhysicsObject)
        (:Is%20Valid
          (Transformation|SetWorldLocation (Variables|/Game/ThirdPersonCPP/Blueprints/BP_Player.BP_Player_C|GetComponentPickupLocation (CallFunction|GetPlayer)) (Transformation|GetWorldLocation (Variables|Default|GetPhysicsObject)) false false)
          (Physics|Components|PhysicsHandle|GrabComponentatLocationwithRotation (Variables|/Game/ThirdPersonCPP/Blueprints/BP_Player.BP_Player_C|GetPhysicsHandle (CallFunction|GetPlayer)) (Variables|Default|GetPhysicsObject) "None" (+ (* (Math|Vector|NegateVector (Math|Vector|GetForwardVector _componentpickuplocation)) (Variables|Default|GetMagForce)) (Transformation|GetWorldLocation _componentpickuplocation)) (Math|Rotator|MakeRotator (.roll _returnvalue) (.pitch _returnvalue) (.yaw _returnvalue)))
          (CallFunction|SetAllItemsOrigin)
          (bind _asbp_item_2 (Utilities|Casting|CastToBP_Item (Components|GetOwner (Variables|Default|GetPhysicsObject)))
            (:then
              (Default|SetMaterialYellow _asbp_item_2))
            (:CastFailed
              (bind _asbp_scene_interactive_2 (Utilities|Casting|CastToBP_SceneInteractive (Components|GetOwner (Variables|Default|GetPhysicsObject))))
              (Default|SetMaterialYellow _asbp_scene_interactive_2)))
          (Variables|Default|SetIsGrabbing true))))))

(event Custom|MagAddForce
  (params (AxisValue :type Float%20%28double-precision%29))
  (Utilities|IsValid (Variables|Default|GetPhysicsObject)
    (:Is%20Valid
      (Variables|Default|SetMagForce (+ (* AxisValue (Variables|Default|GetMagScale)) (Variables|Default|GetMagForce))))))

(event Custom|ViewGrab
  (if (not (Variables|Default|GetIsGrabbing))
    (Utilities|FlowControl|FlipFlop
      (:A
        (CallFunction|SetAllItemsPink))
      (:B
        (CallFunction|SetAllItemsOrigin)))))

(event Custom|RotItemRoll
  (params (Value :type Float%20%28double-precision%29))
  (Variables|Default|SetRotRoll Value))

(event Custom|Attach
  (bind _physicsobject (Variables|Default|GetPhysicsObject))
  (Utilities|IsValid _physicsobject
    (:Is%20Valid
      (bind _asbp_item (Utilities|Casting|CastToBP_Item (Components|GetOwner _physicsobject)))
      (for _array_element (Variables|/Game/Item_System/Item/BP_ItemBase.BP_ItemBase_C|GetAllPoints _asbp_item)
        (Utilities|IsValid _array_element
          (:Is%20Valid
            (for _array_element_2 (Variables|Default|GetAllItemPoints)
              (Utilities|IsValid _array_element_2
                (:Is%20Valid
                  (if (!= _array_element_2 _array_element)
                    (if (and (<= (Math|Vector|Distance(Vector) (Transformation|GetWorldLocation _array_element_2) (Transformation|GetWorldLocation _array_element)) (Variables|Default|GetPointMinDistance)) (!= (Components|GetOwner _array_element) (Components|GetOwner _array_element_2)))
                      (Variables|Default|SetPointMinDistance (Math|Vector|Distance(Vector) (Transformation|GetWorldLocation _array_element_2) (Transformation|GetWorldLocation _array_element)))
                      (bind _asbp_item_2 (Utilities|Casting|CastToBP_Item (Components|GetOwner _array_element_2)))
                      (Variables|Default|SetMinDIstanceObject _asbp_item_2)))))))))
      (Utilities|IsValid (Variables|Default|GetMinDIstanceObject)
        (:Is%20Valid
          (bind _successattach (Default|Attach (Variables|Default|GetMinDIstanceObject) (.AsBP%20Item (Utilities|Casting|CastToBP_Item (Components|GetOwner (Variables|Default|GetPhysicsObject))))))
          (if _successattach
            _))))))

(event Custom|Adsorption
  (bind _physicsobject (Variables|Default|GetPhysicsObject))
  (bind _returnvalue (Components|GetOwner _physicsobject))
  (Utilities|IsValid _physicsobject
    (:Is%20Valid
      (bind _asbp_item (Utilities|Casting|CastToBP_Item _returnvalue))
      (for _array_element (Variables|Default|GetItems)
        (if (!= _array_element _returnvalue)
          (if (<= (Math|Vector|Distance(Vector) (CallFunction|GetMeshLocation _array_element) (CallFunction|GetMeshLocation _asbp_item)) (Variables|Default|GetMinDistance))
            (Variables|Default|SetMinDistance (Math|Vector|Distance(Vector) (CallFunction|GetMeshLocation _array_element) (CallFunction|GetMeshLocation _asbp_item)))
            (Variables|Default|SetMinDIstanceObject _array_element))))
      (Utilities|IsValid (Variables|Default|GetMinDIstanceObject)
        (:Is%20Valid
          (if (not (or (== (Utilities|Array|Length (Variables|/Game/Item_System/Item/BP_ItemBase.BP_ItemBase_C|GetAllPoints (Variables|Default|GetMinDIstanceObject))) 0) (== (Utilities|Array|Length (Variables|/Game/Item_System/Item/BP_ItemBase.BP_ItemBase_C|GetAllPoints (.AsBP%20Item (Utilities|Casting|CastToBP_Item (Components|GetOwner (Variables|Default|GetPhysicsObject)))))) 0)))
            (for _array_element_2 (Variables|/Game/Item_System/Item/BP_ItemBase.BP_ItemBase_C|GetAllPoints (Variables|Default|GetMinDIstanceObject))
              (for _array_element_3 (Variables|/Game/Item_System/Item/BP_ItemBase.BP_ItemBase_C|GetAllPoints (.AsBP%20Item (Utilities|Casting|CastToBP_Item (Components|GetOwner (Variables|Default|GetPhysicsObject)))))
                (if (<= (Math|Vector|Distance(Vector) (Transformation|GetWorldLocation _array_element_3) (Transformation|GetWorldLocation _array_element_2)) (Variables|Default|GetPointMinDistance))
                  (Variables|Default|SetPointMinDistance (Math|Vector|Distance(Vector) (Transformation|GetWorldLocation _array_element_3) (Transformation|GetWorldLocation _array_element_2)))
                  (Variables|Default|SetPointSelf _array_element_3)
                  (Variables|Default|SetPointAnother _array_element_2))))
            (if (Variables|/Game/Item_System/Item/BP_ItemBase.BP_ItemBase_C|GetCanReceiveMesh (Variables|Default|GetMinDIstanceObject))
              (Transformation|SetWorldRotation (Variables|/Game/Item_System/Item/BP_ItemBase.BP_ItemBase_C|GetStaticMesh (.AsBP%20Item (Utilities|Casting|CastToBP_Item (Components|GetOwner (Variables|Default|GetPhysicsObject))))) (Transformation|GetWorldRotation (Variables|Default|GetPointAnother)) false false)
              (Variables|Default|SetPointMinDistance 9999999.0)
              (for _array_element_4 (Variables|/Game/Item_System/Item/BP_ItemBase.BP_ItemBase_C|GetAllPoints (.AsBP%20Item (Utilities|Casting|CastToBP_Item (Components|GetOwner (Variables|Default|GetPhysicsObject)))))
                (if (<= (Math|Vector|Distance(Vector) (Transformation|GetWorldLocation (Variables|Default|GetPointAnother)) (Transformation|GetWorldLocation _array_element_4)) (Variables|Default|GetPointMinDistance))
                  (Variables|Default|SetPointMinDistance (Math|Vector|Distance(Vector) (Transformation|GetWorldLocation (Variables|Default|GetPointAnother)) (Transformation|GetWorldLocation _array_element_4)))
                  (Variables|Default|SetPointSelf _array_element_4)))
              (Default|Combine (Variables|Default|GetMinDIstanceObject) (.AsBP%20Item (Utilities|Casting|CastToBP_Item (Components|GetOwner (Variables|Default|GetPhysicsObject)))) (Variables|Default|GetPointAnother) (Variables|Default|GetPointSelf)))))))))

(event Custom|RotItemPitch
  (params (Value :type Float%20%28double-precision%29))
  (Variables|Default|SetRotPitch Value))

(event Custom|RotItemYaw
  (params (Value :type Float%20%28double-precision%29))
  (Variables|Default|SetRotYaw Value))

(event EventBeginPlay
  (CallFunction|CollectionItems))

(event EventTick
  (params (DeltaSeconds :type Float%20%28single-precision%29))
  (bind _player (CallFunction|GetPlayer))
  (bind _player_2 (CallFunction|GetPlayer))
  (bind _returnvalue (Math|Vector|VectorUp))
  (bind _rotpitch (Variables|Default|GetRotPitch))
  (bind _rotroll (Variables|Default|GetRotRoll))
  (bind _rotyaw (Variables|Default|GetRotYaw))
  (bind _returnvalue_2 (* _rotroll 1.0))
  (bind _returnvalue_3 (* _rotyaw 1.0))
  (bind _returnvalue_4 (* _rotpitch -1.0))
  (bind _physicshandle (Variables|/Game/ThirdPersonCPP/Blueprints/BP_Player.BP_Player_C|GetPhysicsHandle _player_2))
  (bind _componentpickuplocation (Variables|/Game/ThirdPersonCPP/Blueprints/BP_Player.BP_Player_C|GetComponentPickupLocation _player))
  (bind _followcamera (Variables|/Script/SSGame.SSGameCharacter|GetFollowCamera _player_2))
  (bind _returnvalue_5 (Math|Vector|RotatorfromAxisandAngle _returnvalue _returnvalue_3))
  (bind (_targetlocation _targetrotation) (Class|PhysicsHandleComponent|GetTargetLocationandRotation _physicshandle))
  (bind _returnvalue_6 (Transformation|GetWorldLocation _followcamera))
  (bind _returnvalue_7 (- _targetlocation _returnvalue_6))
  (bind _returnvalue_8 (Math|Vector|MakeVector (.x _returnvalue_7) (.y _returnvalue_7) 0.0))
  (bind _returnvalue_9 (Math|Vector|Normalize _returnvalue_8))
  (bind (_x _y) (Math|Vector|BreakVector _returnvalue_9))
  (bind _returnvalue_10 (Math|Vector|RotatorfromAxisandAngle _returnvalue_9 _returnvalue_2))
  (bind _returnvalue_11 (* -1 _x))
  (bind _returnvalue_12 (Math|Vector|MakeVector _y _returnvalue_11 0.0))
  (bind _returnvalue_13 (Math|Vector|RotatorfromAxisandAngle _returnvalue_12 _returnvalue_4))
  (bind _returnvalue_14 (Math|Rotator|CombineRotators _returnvalue_13 _returnvalue_5))
  (bind _returnvalue_15 (Math|Rotator|CombineRotators _returnvalue_10 _returnvalue_14))
  (bind _returnvalue_16 (Math|Rotator|CombineRotators _targetrotation _returnvalue_15))
  (Utilities|IsValid (Variables|Default|GetPhysicsObject)
    (:Is%20Valid
      (Class|PhysicsHandleComponent|SetTargetLocationandRotation _physicshandle (+ (* (Math|Vector|NegateVector (Math|Vector|GetForwardVector _componentpickuplocation)) (Variables|Default|GetMagForce)) (Transformation|GetWorldLocation _componentpickuplocation) (* (Math|Vector|VectorUp) (Variables|Default|GetFlo))) (Math|Rotator|MakeRotator (.roll _returnvalue_16) (.pitch _returnvalue_16) (.yaw _returnvalue_16)))
      (CallFunction|ShowCanAttachItem))))

(fn ActiveMagnesisRune
  (bind _player (CallFunction|GetPlayer))
  (bind _followcamera (Variables|/Script/SSGame.SSGameCharacter|GetFollowCamera _player))
  (bind _returnvalue (Transformation|GetWorldLocation _followcamera))
  (bind (_outhit _returnvalue_2) (Collision|LineTraceByChannel _returnvalue (+ _returnvalue (* (Math|Vector|GetForwardVector _followcamera) (Variables|Default|GetMagnesisDistance))) "TraceTypeQuery1" false 0 "ForDuration"))
  (if _returnvalue_2
    (bind _asbp_item (Utilities|Casting|CastToBP_Item (.HitActor (Collision|BreakHitResult _outhit)))
      (:then
        (if (Variables|/Game/Item_System/Item/BP_ItemBase.BP_ItemBase_C|GetCanGrab _asbp_item)
          (Variables|Default|SetPhysicsObject (.HitComponent (Collision|BreakHitResult _outhit)) :!label _label)
          (bind _asbp_gear_l (Utilities|Casting|CastToBP_GearL _asbp_item)
            (:then
              (Physics|SetSimulatePhysics (Variables|/Game/Item_System/Item/BP_ItemBase.BP_ItemBase_C|GetStaticMesh _asbp_gear_l) true))
            (:CastFailed
              (bind _asbp_item_2 (Utilities|Casting|CastToBP_Item (.HitActor (Collision|BreakHitResult _outhit))))
              (for _array_element (Variables|/Game/Item_System/Item/BP_ItemBase.BP_ItemBase_C|GetAllReceiveItems _asbp_item_2)
                (bind _asbp_gear_l_2 (Utilities|Casting|CastToBP_GearL _array_element))
                (Physics|SetSimulatePhysics (Variables|/Game/Item_System/Item/BP_ItemBase.BP_ItemBase_C|GetStaticMesh _asbp_gear_l_2) true))))))
      (:CastFailed
        (Utilities|Casting|CastToBP_SceneInteractive (.HitActor (Collision|BreakHitResult _outhit)))
        (goto _label)))))

(fn GetPlayer
  (bind _asbp_player (Utilities|Casting|CastToBP_Player (Components|GetOwner))
    (:then
      (return _asbp_player))
    (:CastFailed
      (return 0))))

(fn SetPhysicsMaterial)

(fn SetAllItemsPink
  (bind _outactors (Actor|GetAllActorsOfClass "/Game/Item_System/Item/BP_Item.BP_Item_C"))
  (for _array_element _outactors
    (if (Variables|/Game/Item_System/Item/BP_ItemBase.BP_ItemBase_C|GetCanGrab _array_element)
      (Default|SetMaterialPink _array_element)))
  (bind _outactors_2 (Actor|GetAllActorsOfClass "/Game/Blueprints/BP_SceneInteractive.BP_SceneInteractive_C"))
  (for _array_element_2 _outactors_2
    (Default|SetMaterialPink _array_element_2)))

(fn SetAllItemsOrigin
  (bind _outactors (Actor|GetAllActorsOfClass "/Game/Item_System/Item/BP_Item.BP_Item_C"))
  (for _array_element _outactors
    (Default|SetMaterialOrigin _array_element))
  (bind _outactors_2 (Actor|GetAllActorsOfClass "/Game/Blueprints/BP_SceneInteractive.BP_SceneInteractive_C"))
  (for _array_element_2 _outactors_2
    (Default|SetMaterialOrigin _array_element_2)))

(fn Float
  (if (and (<= (Variables|Default|GetFlo) 25.0) (Variables|Default|GetUp))
    (Variables|Default|SetUp true)
    (Variables|Default|SetDown false)
    (else
      (Variables|Default|SetDown true)
      (Variables|Default|SetUp false)))
  (if (Variables|Default|GetUp)
    (Variables|Default|SetFlo (+ (Variables|Default|GetFlo) 0.3))
    (else
      (Variables|Default|SetFlo (- (Variables|Default|GetFlo) 0.3))))
  (if (and (>= (Variables|Default|GetFlo) -25.0) (Variables|Default|GetDown))
    (Variables|Default|SetDown true)
    (Variables|Default|SetUp false)
    (else
      (Variables|Default|SetUp true)
      (Variables|Default|SetDown false))))

(fn GetMeshLocation
  (params (Item :type BP%20Item%20Object%20Reference))
  (switch Utilities|FlowControl|Switch|SwitchonMeshType (CallFunction|GetMeshType (Utilities|Struct|BreakPackage_Info (Variables|/Game/Item_System/Item/BP_ItemBase.BP_ItemBase_C|GetPackage_Info Item)))
    (:NewEnumerator0
      (return (Transformation|GetWorldLocation (Variables|/Game/Item_System/Item/BP_ItemBase.BP_ItemBase_C|GetSkeletalMesh Item))))
    (:NewEnumerator1
      (return (Transformation|GetWorldLocation (Variables|/Game/Item_System/Item/BP_ItemBase.BP_ItemBase_C|GetStaticMesh Item))))))

(fn GetCouldCombineActors
  (bind _outactors (Actor|GetAllActorsOfClass "/Game/Item_System/Item/BP_Item.BP_Item_C"))
  (for _array_element _outactors
    (if (Variables|/Game/Item_System/Item/BP_ItemBase.BP_ItemBase_C|GetCanReceiveMesh _array_element)
      (Utilities|Array|Add (Variables|Default|GetItems) _array_element))))

(fn GetAllItems
  (Utilities|Array|Clear (Variables|Default|GetAllItemPoints))
  (bind _outactors (Actor|GetAllActorsOfClass "/Game/Item_System/Item/BP_Item.BP_Item_C"))
  (for _array_element _outactors
    (Utilities|Array|Add (Variables|Default|GetItems) _array_element)
    (for _array_element_2 (Variables|/Game/Item_System/Item/BP_ItemBase.BP_ItemBase_C|GetAllPoints _array_element)
      (Utilities|Array|Add (Variables|Default|GetAllItemPoints) _array_element_2))))

(fn ShowCanAttachItem
  (bind _physicsobject (Variables|Default|GetPhysicsObject))
  (Utilities|IsValid _physicsobject
    (:Is%20Valid
      (bind _asbp_item (Utilities|Casting|CastToBP_Item (Components|GetOwner _physicsobject)))
      (bind _points (CallFunction|GetCloseItemPoints _asbp_item))
      (for _array_element (Variables|/Game/Item_System/Item/BP_ItemBase.BP_ItemBase_C|GetAllPoints _asbp_item)
        (Utilities|IsValid _array_element
          (:Is%20Valid
            (for _array_element_2 _points
              (Utilities|IsValid _array_element_2
                (:Is%20Valid
                  (if (!= _array_element_2 _array_element)
                    (if (and (<= (Math|Vector|Distance(Vector) (Transformation|GetWorldLocation _array_element_2) (Transformation|GetWorldLocation _array_element)) (Variables|Default|GetTempPointMinDistance)) (!= (Components|GetOwner _array_element) (Components|GetOwner _array_element_2)))
                      (Variables|Default|SetTempPointMinDistance (Math|Vector|Distance(Vector) (Transformation|GetWorldLocation _array_element_2) (Transformation|GetWorldLocation _array_element)))
                      (bind _asbp_item_2 (Utilities|Casting|CastToBP_Item (Components|GetOwner _array_element_2)))
                      (Variables|Default|SetTempMinObject _asbp_item_2)))))))))
      (Variables|Default|SetTempPointMinDistance (Variables|Default|GetInitialPointMinDistance))
      (bind _asbp_item_3 (Utilities|Casting|CastToBP_Item (Components|GetOwner (Variables|Default|GetPhysicsObject))))
      (CallFunction|ShowNearestPoints _asbp_item_3 (Variables|Default|GetTempMinObject))
      (Variables|Default|SetTempMinObject 0))
    (:Is%20Not%20Valid
      (Variables|Default|SetTempPointMinDistance (Variables|Default|GetInitialPointMinDistance)))))

(fn ShowNearestPoints
  (params (ItemA :type BP%20Item%20Object%20Reference) (ItemB :type BP%20Item%20Object%20Reference))
  (Utilities|IsValid ItemA
    (:Is%20Valid
      (Utilities|IsValid ItemB
        (:Is%20Valid
          (LocalVariables|SetPrePointB (Transformation|GetActorLocation ItemA))
          (Utilities|FlowControl|ForLoopwithBreak 0 20 :!label _label
            (:LoopBody
              (if (> (Math|Vector|Distance(Vector) (LocalVariables|GetPrePointA) (.OutPointOnBody (Collision|GetClosestPointonCollision (Variables|/Game/Item_System/Item/BP_ItemBase.BP_ItemBase_C|GetStaticMesh ItemB) (LocalVariables|GetPrePointB) "None"))) 1.0)
                (LocalVariables|SetPrePointA (.OutPointOnBody (Collision|GetClosestPointonCollision (Variables|/Game/Item_System/Item/BP_ItemBase.BP_ItemBase_C|GetStaticMesh ItemB) (LocalVariables|GetPrePointB) "None")))
                (LocalVariables|SetPrePointB (.OutPointOnBody (Collision|GetClosestPointonCollision (Variables|/Game/Item_System/Item/BP_ItemBase.BP_ItemBase_C|GetStaticMesh ItemA) (LocalVariables|GetPrePointA) "None")))
                (else
                  (goto _label Break))))
            (:Completed
              (Rendering|Debug|DrawDebugLine (LocalVariables|GetPrePointA) (LocalVariables|GetPrePointB) "(R=0.071405,G=1.000000,B=0.000000,A=1.000000)" 0.0 4.0))))))))

(fn GetNearestLine
  (params (ItemA :type BP%20Item%20Object%20Reference) (ItemB :type BP%20Item%20Object%20Reference))
  (LocalVariables|SetPrePointA "10000.000000,10000.000000,10000.000000")
  (Utilities|IsValid ItemA
    (:Is%20Valid
      (Utilities|IsValid ItemB
        (:Is%20Valid
          (LocalVariables|SetPrePointB (Transformation|GetActorLocation ItemA))
          (Utilities|FlowControl|ForLoopwithBreak 0 20 :!label _label
            (:LoopBody
              (if (> (Math|Vector|Distance(Vector) (LocalVariables|GetPrePointA) (.OutPointOnBody (Collision|GetClosestPointonCollision (Variables|/Game/Item_System/Item/BP_ItemBase.BP_ItemBase_C|GetStaticMesh ItemB) (LocalVariables|GetPrePointB) "None"))) 1.0)
                (LocalVariables|SetPrePointA (.OutPointOnBody (Collision|GetClosestPointonCollision (Variables|/Game/Item_System/Item/BP_ItemBase.BP_ItemBase_C|GetStaticMesh ItemB) (LocalVariables|GetPrePointB) "None")))
                (LocalVariables|SetPrePointB (.OutPointOnBody (Collision|GetClosestPointonCollision (Variables|/Game/Item_System/Item/BP_ItemBase.BP_ItemBase_C|GetStaticMesh ItemA) (LocalVariables|GetPrePointA) "None")))
                (else
                  (goto _label Break))))
            (:Completed
              (return (LocalVariables|GetPrePointA) (LocalVariables|GetPrePointB)))))))))

(fn CollectionItems
  (CallFunction|GetAllItems)
  (bind _outactors (Actor|GetAllActorsOfClass "/Game/Blueprints/BP_SceneInteractive.BP_SceneInteractive_C"))
  (for _array_element _outactors
    (for _array_element_2 (Actor|GetComponentsByClass _array_element "/Script/Engine.StaticMeshComponent")
      (if (Physics|IsSimulatingPhysics _array_element_2 "None")
        (Utilities|Array|Add (Variables|Default|GetSceneCanInteractiveMeshes) _array_element_2)))))

(fn GetCloseItemPoints
  (params (Item :type BP%20Item%20Object%20Reference))
  (bind _asbp_player (Utilities|Casting|CastToBP_Player (Game|GetPlayerCharacter 0)))
  (for _array_element (Variables|/Game/ThirdPersonCPP/Blueprints/BP_Player.BP_Player_C|GetAllItems _asbp_player)
    (Utilities|IsValid _array_element
      (:Is%20Valid
        (if (< (Transformation|GetDistanceTo _array_element Item) 3e+02)
          (for _array_element_2 (Variables|/Game/Item_System/Item/BP_ItemBase.BP_ItemBase_C|GetAllPoints _array_element)
            (Utilities|Array|Add (LocalVariables|GetAllPoints) _array_element_2))))))
  (return (LocalVariables|GetAllPoints)))