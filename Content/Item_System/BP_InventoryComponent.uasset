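; Inventory component for the player pawn that stores items in a grid bag, where each item occupies a rectangle of cells.
; Pushing an item scans a flattened cell array for the first free fit, retrying once with the item rotated.
; Adding and removing set a dirty flag, which Tick turns into an OnBagChanged call.
; It also creates and toggles the main UI widget and spawns dropped items in front of the pawn.
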(event Custom|OpenAndCloseBag
  (bind _playercontroller (Variables|Default|GetPlayerController))
  (bind _playercontroller_2 (Variables|Default|GetPlayerController))
  (if (Widget|IsVisible (Variables|Default|GetMainUI))
    (Widget|RemovefromParent (Variables|Default|GetMainUI))
    (Variables|/Script/Engine.PlayerController|SetbShowMouseCursor _playercontroller false)
    (Input|SetInputModeGameOnly _playercontroller)
    (else
      (UserInterface|Viewport|AddtoViewport (Variables|Default|GetMainUI) 0)
      (Variables|/Script/Engine.PlayerController|SetbShowMouseCursor _playercontroller_2 true)
      (Input|SetInputModeGameandUI _playercontroller_2 (Variables|Default|GetMainUI) "DoNotLock" false))))

(event EventBeginPlay
  (Utilities|FlowControl|Sequence
    (:then_0
      (bind _aspawn (Utilities|Casting|CastToPawn (Components|GetOwner)))
      (Variables|Default|SetAs%20Pawn _aspawn)
      (bind _asbp_player_controller (Utilities|Casting|CastToBP_PlayerController (Pawn|GetController _aspawn)))
      (Variables|Default|SetPlayerController _asbp_player_controller)
      (bind _asbp_player (Utilities|Casting|CastToBP_Player _aspawn))
      (Variables|Default|SetMyPlayer _asbp_player))
    (:then_1
      (bind _returnvalue (UserInterface|CreateWidget "/Game/Item_System/UI/WBP_MainUI.WBP_MainUI_C" (Variables|Default|GetPlayerController) (Variables|/Game/ThirdPersonCPP/Blueprints/BP_Player.BP_Player_C|GetBP_InventoryComponent (Variables|Default|GetMyPlayer)) (Variables|Default|GetCellSize)))
      (Variables|Default|SetMainUI _returnvalue))
    (:then_2
      (Utilities|Array|Resize (Variables|Default|GetItemInventory) (* (Variables|Default|GetColums) (Variables|Default|GetRows))))))

(event EventTick
  (params (DeltaSeconds :type Float%20%28single-precision%29))
  (if (Variables|Default|GetBagChanged)
    (Default|CallOnBagChanged)
    (Variables|Default|SetBagChanged false)))

(fn BeginPushIteminBag
  (params (ItemObject :type BP%20Item%20Object%20Object%20Reference))
  (Utilities|IsValid ItemObject
    (:Is%20Valid
      (Variables|Default|SetItem%20Object ItemObject)
      (for (_ _array_index) (Variables|Default|GetItemInventory) :!label _label
        (bind _ishasenoughspace (CallFunction|IsHasEnoughSpace ItemObject _array_index))
        (if _ishasenoughspace
          (CallFunction|AddItem ItemObject _array_index)
          (return true)))
      (Utilities|FlowControl|Sequence
        (:then_0
          (Utilities|FlowControl|DoOnce false
            (:Completed
              (Default|Rotation (Variables|Default|GetItem%20Object))
              (goto _label))))
        (:then_1
          (return false))))))

(fn IsHasEnoughSpace
  (params (ItemObject :type BP%20Item%20Object%20Object%20Reference) (TopLeftIndex :type Integer))
  (Utilities|FlowControl|Sequence
    (:then_0
      (bind _tlip (Utilities|LoopIndex (CallFunction|TransGridIndextoLocation TopLeftIndex) ItemObject)
        (:LoopBody
          (Utilities|IsGridEffective _tlip
            (:true
              (bind _iseffective (CallFunction|IsCurrentIndexEffective (CallFunction|TransGridLocationtoIndex _tlip)))
              (if (not _iseffective)
                (return false)))
            (:false
              (return false))))))
    (:then_1
      (return true))))

(fn AddItem
  (params (ItemObject :type BP%20Item%20Object%20Object%20Reference) (TopLeftIndex :type Integer))
  (bind _tlip (Utilities|LoopIndex (CallFunction|TransGridIndextoLocation TopLeftIndex) ItemObject)
    (:LoopBody
      (Utilities|Array|SetArrayElem (Variables|Default|GetItemInventory) (CallFunction|TransGridLocationtoIndex _tlip) ItemObject))
    (:Completed
      (Variables|Default|SetBagChanged true))))

(fn TransGridLocationtoIndex
  (params (TopLeftTlip :type Tlip%20Structure))
  (bind (_x _y) (Utilities|Struct|BreakTlip TopLeftTlip))
  (return (+ _x (* _y (Variables|Default|GetColums)))))

(fn TransGridIndextoLocation
  (params (TopLeftIndex :type Integer))
  (return (Utilities|Struct|MakeTlip (Math|Integer|%(Integer) TopLeftIndex (Variables|Default|GetColums)) (/ TopLeftIndex (Variables|Default|GetColums)))))

(fn IsCurrentIndexEffective
  (params (Index :type Integer))
  (if (Utilities|Array|IsValidIndex (Variables|Default|GetItemInventory) Index)
    (if (Utilities|IsValid (Utilities|Array|Get(acopy) (Variables|Default|GetItemInventory) Index))
      (return false)
      (else
        (return true)))
    (else
      (return false))))

(fn GetAllItem
  (for (_array_element _array_index) (Variables|Default|GetItemInventory)
    (bind _output_get (LocalVariables|SetCurrentItemObject _array_element))
    (Utilities|IsValid _output_get
      (:Is%20Valid
        (if (not (Utilities|Map|Contains (LocalVariables|GetItems) _output_get))
          (Utilities|Map|Add (LocalVariables|GetItems) (LocalVariables|GetCurrentItemObject) (CallFunction|TransGridIndextoLocation _array_index))))))
  (return (LocalVariables|GetItems)))

(fn RemoveItem
  (params (ItemObject :type BP%20Item%20Object%20Object%20Reference))
  (Utilities|IsValid ItemObject
    (:Is%20Valid
      (for (_array_element _array_index) (Variables|Default|GetItemInventory)
        (if (== _array_element ItemObject)
          (Utilities|Array|SetArrayElem (Variables|Default|GetItemInventory) _array_index 0)))
      (Variables|Default|SetBagChanged true)
      (return))
    (:Is%20Not%20Valid
      (return))))

(fn DropandSpawnItem
  (params (ItemObject :type BP%20Item%20Object%20Object%20Reference))
  (bind _as_pawn (Variables|Default|GetAs%20Pawn))
  (bind _as_pawn_2 (Variables|Default|GetAs%20Pawn))
  (bind _returnvalue (Pawn|GetControlRotation _as_pawn_2 :!class /Script/Engine.Pawn))
  (Game|SpawnActorfromClass (Utilities|Struct|BreakPackage_Info (Default|GetPackageInfo ItemObject)) (Math|Transform|MakeTransform (+ (Transformation|GetActorLocation _as_pawn) (* (Transformation|GetActorForwardVector _as_pawn) 1e+02)) (Math|Rotator|MakeRotator (.roll _returnvalue) 0.0 (.yaw _returnvalue)) "1,1,1") "Undefined" 0 (Default|GetPackageInfo ItemObject) 0)
  (CallFunction|RemoveItem ItemObject)
  (return))