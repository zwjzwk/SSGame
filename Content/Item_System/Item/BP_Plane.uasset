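; BP_Plane is a combinable item that serves as a plane body with four mount points for BP_Fan items.
; Combine calls the parent, then stores an attached fan in the PlaneFans slot matching its mount point.
; Forward/back and left/right force events write input magnitudes into InputValues pairs chosen by sign, with positive left/right using index 4 rather than 3.
; BeginPlay sets high angular damping on the mesh, and nothing here applies InputValues to the fans.
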(event Custom|SetForceFAndB
  (params (Value :type Float%20%28double-precision%29))
  (bind _returnvalue (* Value -1.0))
  (if (> Value 0.0)
    (Utilities|Array|SetArrayElem (Variables|Default|GetInputValues) 2 Value)
    (Utilities|Array|SetArrayElem (Variables|Default|GetInputValues) 3 Value)
    (else
      (Utilities|Array|SetArrayElem (Variables|Default|GetInputValues) 0 _returnvalue)
      (Utilities|Array|SetArrayElem (Variables|Default|GetInputValues) 1 _returnvalue))))

(event Custom|SetForceLAndR
  (params (Value :type Float%20%28double-precision%29))
  (bind _returnvalue (* Value -1.0))
  (if (> Value 0.0)
    (Utilities|Array|SetArrayElem (Variables|Default|GetInputValues) 1 Value)
    (Utilities|Array|SetArrayElem (Variables|Default|GetInputValues) 4 Value)
    (else
      (Utilities|Array|SetArrayElem (Variables|Default|GetInputValues) 0 _returnvalue)
      (Utilities|Array|SetArrayElem (Variables|Default|GetInputValues) 2 _returnvalue))))

(event EventBeginPlay
  (|CallParentFunction)
  (Class|PrimitiveComponent|SetAngularDamping (Variables|Default|GetStaticMesh) 3e+01))

(event EventTick
  (params (DeltaSeconds :type Float%20%28single-precision%29))
  (|CallParentFunction DeltaSeconds))

(fn ConstructionScript
  (|CallParentFunction))

(fn AddMesh
  (params (AnotherItem :type BP%20Item%20Object%20Reference) (PointMain :type Scene%20Component%20Object%20Reference) (Material :type Material%20Interface%20Object%20Reference) (PointGrab :type Scene%20Component%20Object%20Reference))
  (bind (_success _mesh) (|CallParentFunction AnotherItem PointMain Material PointGrab))
  (return _success _mesh))

(fn Combine
  (params (AnotherItem :type BP%20Item%20Object%20Reference) (PointMain :type Scene%20Component%20Object%20Reference) (PointGrab :type Scene%20Component%20Object%20Reference))
  (|CallParentFunction AnotherItem PointMain PointGrab)
  (bind _asbp_fan (Utilities|Casting|CastToBP_Fan AnotherItem))
  (Utilities|FlowControl|Sequence
    (:then_0
      (if (== (Variables|Default|GetScene3) PointMain)
        (Utilities|Array|SetArrayElem (Variables|Default|GetPlaneFans) 0 _asbp_fan)))
    (:then_1
      (if (== (Variables|Default|GetScene) PointMain)
        (Utilities|Array|SetArrayElem (Variables|Default|GetPlaneFans) 1 _asbp_fan)))
    (:then_2
      (if (== (Variables|Default|GetScene1) PointMain)
        (Utilities|Array|SetArrayElem (Variables|Default|GetPlaneFans) 2 _asbp_fan)))
    (:then_3
      (if (== (Variables|Default|GetScene2) PointMain)
        (Utilities|Array|SetArrayElem (Variables|Default|GetPlaneFans) 3 _asbp_fan)))))