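; Item inspection actor that shows a picked item's mesh in a preview UI, where the player rotates and zooms it.
; CreateItemRender takes input from the player, sets mesh, material and scale from the package ID, scales camera arm length by item size and opens the render widget.
; A scene capture shows only this actor.
; Pickup bags the item and ExitView leaves it; both restore player input and destroy the actor.
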(event Custom|SetMesh
  (bind _package_info (Variables|Default|GetPackage%20Info))
  (bind _springarm (Variables|Default|GetSpringArm))
  (bind _staticmesh (Variables|Default|GetStaticMesh))
  (bind _package_info_2 (Variables|Default|GetPackage%20Info))
  (bind _skeletalmesh (Variables|Default|GetSkeletalMesh))
  (bind _id (Utilities|Struct|BreakPackage_Info _package_info))
  (bind _id_2 (Utilities|Struct|BreakPackage_Info _package_info_2))
  (bind _itemscale (CallFunction|GetItemScale _id_2))
  (bind _material (CallFunction|GetMaterial _id))
  (switch Utilities|FlowControl|Switch|SwitchonMeshType (CallFunction|GetMeshType (.ID (Utilities|Struct|BreakPackage_Info (Variables|Default|GetPackage%20Info))))
    (:NewEnumerator0
      (Class|SkinnedMeshComponent|SetSkeletalMesh _skeletalmesh (CallFunction|GetSkeletalMesh _id) true)
      (Rendering|Material|SetMaterial _skeletalmesh 0 _material)
      (Transformation|SetWorldScale3D _skeletalmesh _itemscale))
    (:NewEnumerator1
      (Components|StaticMesh|SetStaticMesh _staticmesh (CallFunction|GetStaticMesh _id))
      (Rendering|Material|SetMaterial _staticmesh 0 _material)
      (Transformation|SetWorldScale3D _staticmesh _itemscale)))
  (Variables|/Script/Engine.SpringArmComponent|SetTargetArmLength _springarm (* (/ (Math|Vector|VectorLength (CallFunction|GetItemScale (Utilities|Struct|BreakPackage_Info (Variables|Default|GetPackage%20Info)))) 2.0) (Variables|/Script/Engine.SpringArmComponent|GetTargetArmLength _springarm))))

(event Custom|RotateSkeletalMesh%28Vertical%29
  (params (Vertical :type Float%20%28single-precision%29))
  (Transformation|SetWorldRotation (Variables|Default|GetSkeletalMesh) (Math|Rotator|CombineRotators (Transformation|GetWorldRotation (Variables|Default|GetSkeletalMesh)) (Math|Rotator|MakeRotator 0.0 (* Vertical -1.0) 0.0)) false false))

(event Custom|RotateSkeletalMesh%28Horizaontal%29
  (params (Horizontal :type Float%20%28single-precision%29))
  (Transformation|SetWorldRotation (Variables|Default|GetSkeletalMesh) (Math|Rotator|CombineRotators (Transformation|GetWorldRotation (Variables|Default|GetSkeletalMesh)) (Math|Rotator|MakeRotator 0.0 0.0 (* Horizontal -1.0))) false false))

(event Custom|RotateStaticMesh%28Vertival%29
  (params (Vertical :type Float%20%28single-precision%29))
  (Transformation|SetWorldRotation (Variables|Default|GetStaticMesh) (Math|Rotator|CombineRotators (Transformation|GetWorldRotation (Variables|Default|GetStaticMesh)) (Math|Rotator|MakeRotator 0.0 (* Vertical -1.0) 0.0)) false false))

(event Custom|RotateStaticMesh%28Horizantal%29
  (params (Horizontal :type Float%20%28single-precision%29))
  (Transformation|SetWorldRotation (Variables|Default|GetStaticMesh) (Math|Rotator|CombineRotators (Transformation|GetWorldRotation (Variables|Default|GetStaticMesh)) (Math|Rotator|MakeRotator 0.0 0.0 (* Horizontal -1.0))) false false))

(event Custom|RotateSkeletalMesh%28c%29
  (params (Value :type Float%20%28single-precision%29))
  (Transformation|SetWorldRotation (Variables|Default|GetSkeletalMesh) (Math|Rotator|CombineRotators (Transformation|GetWorldRotation (Variables|Default|GetSkeletalMesh)) (Math|Rotator|MakeRotator (* Value -1.0) 0.0 0.0)) false false))

(event Custom|RotateStaticMesh%28c%29
  (params (Value :type Float%20%28single-precision%29))
  (Transformation|SetWorldRotation (Variables|Default|GetStaticMesh) (Math|Rotator|CombineRotators (Transformation|GetWorldRotation (Variables|Default|GetStaticMesh)) (Math|Rotator|MakeRotator (* Value -1.0) 0.0 0.0)) false false))

(event EventCreateItemRender
  (params (Item :type BP%20Item%20Base%20Object%20Reference) (MyPlayer :type BP%20Player%20Object%20Reference) (PackageInfo :type Package%20Info%20Structure))
  (Variables|Default|SetItem Item)
  (bind _output_get (Variables|Default|SetMy%20Player MyPlayer))
  (Variables|Default|SetMyPlayerController (.AsBP%20Player%20Controller (Utilities|Casting|CastToBP_PlayerController (Pawn|GetController _output_get))))
  (Variables|Default|SetPackage%20Info PackageInfo)
  (Input|EnableInput (Variables|Default|GetMyPlayerController))
  (Input|DisableInput (Variables|Default|GetMy%20Player) (Variables|Default|GetMyPlayerController))
  (CallFunction|SetMesh)
  (bind _returnvalue (UserInterface|CreateWidget "/Game/Item_System/Item/Item_Render/WBP_ItemRenderUI.WBP_ItemRenderUI_C" (Variables|Default|GetMyPlayerController)))
  (bind _output_get_2 (Variables|Default|SetRenderUI _returnvalue))
  (UserInterface|Viewport|AddtoViewport _output_get_2 0))

(event Input|ActionEvents|InputActionPickup
  (params (Key :type Key%20Structure :default "None"))
  (:Pressed
    (Default|PushBag (Variables|Default|GetItem))
    (Input|EnableInput (Variables|Default|GetMy%20Player) (Variables|Default|GetMyPlayerController))
    (Input|DisableInput (Variables|Default|GetMyPlayerController))
    (Widget|RemovefromParent (Variables|Default|GetRenderUI))
    (Variables|Default|SetRenderUI 0)
    (Actor|DestroyActor)))

(event Input|ActionEvents|InputActionExitView
  (params (Key :type Key%20Structure :default "None"))
  (:Pressed
    (Default|ExitView (Variables|Default|GetItem))
    (Input|EnableInput (Variables|Default|GetMy%20Player) (Variables|Default|GetMyPlayerController))
    (Input|DisableInput (Variables|Default|GetMyPlayerController))
    (Widget|RemovefromParent (Variables|Default|GetRenderUI))
    (Variables|Default|SetRenderUI 0)
    (Actor|DestroyActor)))

(event Input|AxisEvents|InputAxisMoveForward
  (params (AxisValue :type Float%20%28single-precision%29))
  (if (!= AxisValue 0.0)
    (Variables|Default|SetVertical AxisValue)
    (switch Utilities|FlowControl|Switch|SwitchonMeshType (CallFunction|GetMeshType (.ID (Utilities|Struct|BreakPackage_Info (Variables|Default|GetPackage%20Info))))
      (:NewEnumerator0
        (CallFunction|RotateSkeletalMesh(Vertical) (Variables|Default|GetVertical)))
      (:NewEnumerator1
        (CallFunction|RotateStaticMesh(Vertival) (Variables|Default|GetVertical))))))

(event Input|AxisEvents|InputAxisMoveRight
  (params (AxisValue :type Float%20%28single-precision%29))
  (if (!= AxisValue 0.0)
    (Variables|Default|SetHorizontal AxisValue)
    (switch Utilities|FlowControl|Switch|SwitchonMeshType (CallFunction|GetMeshType (.ID (Utilities|Struct|BreakPackage_Info (Variables|Default|GetPackage%20Info))))
      (:NewEnumerator0
        (CallFunction|RotateSkeletalMesh(Horizaontal) (Variables|Default|GetHorizontal)))
      (:NewEnumerator1
        (CallFunction|RotateStaticMesh(Horizantal) (Variables|Default|GetHorizontal))))))

(event Input|AxisEvents|InputAxisRotItemRoll
  (params (AxisValue :type Float%20%28single-precision%29))
  (if (!= AxisValue 0.0)
    (Variables|Default|SetRot AxisValue)
    (switch Utilities|FlowControl|Switch|SwitchonMeshType (CallFunction|GetMeshType (Utilities|Struct|BreakPackage_Info (Variables|Default|GetPackage%20Info)))
      (:NewEnumerator0
        (CallFunction|RotateSkeletalMesh(c) (Variables|Default|GetRot)))
      (:NewEnumerator1
        (CallFunction|RotateStaticMesh(c) (Variables|Default|GetRot))))))

(event Input|MouseEvents|MouseWheelAxis
  (params (AxisValue :type Float%20%28single-precision%29))
  (bind _springarm (Variables|Default|GetSpringArm))
  (Variables|/Script/Engine.SpringArmComponent|SetTargetArmLength _springarm (+ (* AxisValue (Variables|Default|GetCameraScale)) (Variables|/Script/Engine.SpringArmComponent|GetTargetArmLength _springarm))))

(fn ConstructionScript
  (Rendering|SceneCapture|ShowOnlyActorComponents (Variables|Default|GetSceneCaptureComponent2D) self true))