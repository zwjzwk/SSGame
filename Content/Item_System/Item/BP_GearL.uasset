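; BP_GearL is a gear item that the player switches on and off to make it spin.
; A sphere overlap stores the nearby BP_Player, and the Interaction input toggles Active only while that player is present and the gear has attached or received items.
; While active, Tick turns off physics on the root mesh and rotates it a fixed step per frame, independent of delta time.
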(event OnComponentBeginOverlap(Sphere)
  (params (OverlappedComponent :type Primitive%20Component%20Object%20Reference) (OtherActor :type Actor%20Object%20Reference) (OtherComp :type Primitive%20Component%20Object%20Reference) (OtherBodyIndex :type Integer) (bFromSweep :type Boolean) (SweepResult :type Hit%20Result%20Structure%20%28by%20ref%29))
  (bind _asbp_player (Utilities|Casting|CastToBP_Player OtherActor))
  (Variables|Default|SetSelfPlayer _asbp_player))

(event OnComponentEndOverlap(Sphere)
  (params (OverlappedComponent :type Primitive%20Component%20Object%20Reference) (OtherActor :type Actor%20Object%20Reference) (OtherComp :type Primitive%20Component%20Object%20Reference) (OtherBodyIndex :type Integer))
  (Utilities|Casting|CastToBP_Player OtherActor)
  (Variables|Default|SetSelfPlayer 0))

(event EventBeginPlay
  (|CallParentFunction) ; This node is disabled and will not be called.\nDrag off pins to build functionality.
)

(event Collision|EventActorBeginOverlap
  (params (OtherActor :type Actor%20Object%20Reference))
  (|CallParentFunction OtherActor) ; This node is disabled and will not be called.\nDrag off pins to build functionality.
)

(event EventTick
  (params (DeltaSeconds :type Float%20%28single-precision%29))
  (bind _rootstaticmesh (Variables|Default|GetRootStaticmesh))
  (|CallParentFunction DeltaSeconds)
  (if (Variables|Default|GetActive)
    (Physics|SetSimulatePhysics _rootstaticmesh false)
    (Transformation|AddLocalRotation _rootstaticmesh "0.000000,1.000000,0.000000" false false)))

(event Input|ActionEvents|InputActionInteraction
  (params (Key :type Key%20Structure))
  (:Pressed
    (Utilities|IsValid (Variables|Default|GetSelfPlayer)
      (:Is%20Valid
        (if (or (!= (Utilities|Array|Length (Variables|Default|GetAllAttachedToItems)) 0) (!= (Utilities|Array|Length (Variables|Default|GetAllReceiveItems)) 0))
          (Variables|Default|SetActive (not (Variables|Default|GetActive))))))))

(fn ConstructionScript
  (|CallParentFunction))