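; BP_LaserEmitter is a laser emitter item that traces a light beam forward from its Arrow component.
; Tick passes through a short Delay, then calls CastLight with the arrow's location, direction and a cast distance.
; CastLight runs a complex line trace on a custom channel, visible only as a debug line.
; Hit handling is unfinished: a hit triggers nothing, a miss clears a continue flag, and a face-material check sits unconnected.
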(event EventBeginPlay
  (|CallParentFunction) ; This node is disabled and will not be called.\nDrag off pins to build functionality.
)

(event Collision|EventActorBeginOverlap
  (params (OtherActor :type Actor%20Object%20Reference))
  (|CallParentFunction OtherActor) ; This node is disabled and will not be called.\nDrag off pins to build functionality.
)

(event EventTick
  (params (DeltaSeconds :type Float%20%28single-precision%29))
  (bind _arrow (Variables|Default|GetArrow))
  (|CallParentFunction DeltaSeconds)
  (Utilities|FlowControl|Delay 0.01)
  (CallFunction|CastLight (Transformation|GetWorldLocation _arrow) (Math|Vector|GetForwardVector _arrow) (Variables|Default|GetCastDistance)))

(fn ConstructionScript
  (|CallParentFunction))

(fn CastLight
  (params (CastOrigin :type Vector) (CastDirection :type Vector) (CastDistance :type Float%20%28double-precision%29))
  (LocalVariables|SetL_CastOrigin CastOrigin)
  (LocalVariables|SetL_CastDirection CastDirection)
  (LocalVariables|SetL_CastDistance CastDistance)
  (bind (_outhit _returnvalue) (Collision|LineTraceByChannel (LocalVariables|GetL_CastOrigin) (+ (LocalVariables|GetL_CastOrigin) (* (LocalVariables|GetL_CastDirection) (LocalVariables|GetL_CastDistance))) "TraceTypeQuery3" true 0 "ForDuration" true "(R=1.000000,G=0.000000,B=0.000000,A=1.000000)" "(R=0.000000,G=1.000000,B=0.000000,A=1.000000)" 0.1))
  (if _returnvalue
    (if (not true)
      (LocalVariables|SetL_Continue false :!label _label))
    (else
      (goto _label))))