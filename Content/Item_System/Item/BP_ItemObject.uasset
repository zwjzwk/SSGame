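; BP_ItemObject is an item object in the item system that can be rotated between two orientations.
; Rotation toggles the IsRot flag, which GetSize uses to swap the X and Y dimensions and GetImage uses to pick ImageY over ImageX.
; Rotated art comes from a separate pre-made image, and GetPackageInfo exposes the stored PackageInfo unchanged.
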(fn Rotation
  (Variables|Default|SetIsRot? (not (Variables|Default|GetIsRot?))))

(fn GetImage
  (return (select (Variables|Default|GetIsRot?) (Variables|Default|GetImageY) (Variables|Default|GetImageX))))

(fn GetSize
  (bind _size (Variables|Default|GetSize))
  (bind _size_2 (Variables|Default|GetSize))
  (if (Variables|Default|GetIsRot?)
    (return (Utilities|Struct|MakeIntPoint (.y _size) (.x _size)))
    (else
      (return (Utilities|Struct|MakeIntPoint (.x _size_2) (.y _size_2))))))

(fn GetPackageInfo
  (return (Variables|Default|GetPackage_Info)))