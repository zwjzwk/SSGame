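; BP_LaserRed is a red laser emitter item that bounces its beam off mirrors to trigger laser sensors.
; BeginPlay applies the physics setting and caches initial materials; Tick, throttled by a short Delay, casts from the Arrow component.
; CastLight line-traces in a loop, reflecting off mirror actors and registering itself on any sensor hit after clearing the previous one.
; It destroys and respawns a BP_LightBeamRed actor per segment on every cast.
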(event EventBeginPlay
  (Physics|SetSimulatePhysics (Variables|Default|GetRootStaticmesh) (Variables|Default|GetSimulate))
  (for _array_element (Actor|GetComponentsByClass "/Script/Engine.MeshComponent")
    (for _array_element_2 (Rendering|Material|GetMaterials _array_element)
      (Utilities|Array|Add (Variables|Default|GetInitialMaterials) _array_element_2))))

(event Collision|EventActorBeginOverlap
  (params (OtherActor :type Actor%20Object%20Reference))
  (|CallParentFunction OtherActor) ; This node is disabled and will not be called.\nDrag off pins to build functionality.
)

(event EventTick
  (params (DeltaSeconds :type Float%20%28single-precision%29))
  (bind _arrow (Variables|Default|GetArrow))
  (|CallParentFunction DeltaSeconds)
  (Utilities|FlowControl|Delay 0.01)
  (CallFunction|CastLight (Transformation|GetWorldLocation _arrow) (Math|Vector|GetForwardVector _arrow) (Variables|Default|GetCastDistance)))

(fn ConstructionScript
  (|CallParentFunction))

(fn CastLight
  (params (CastOrigin :type Vector) (CastDirection :type Vector) (CastDistance :type Float%20%28double-precision%29))
  (LocalVariables|SetL_CastOrigin CastOrigin)
  (LocalVariables|SetL_CastDirection CastDirection)
  (LocalVariables|SetL_CastDistance CastDistance)
  (for _array_element (Variables|Default|GetBeams)
    (Actor|DestroyActor _array_element))
  (Utilities|Array|Clear (Variables|Default|GetBeams))
  (Utilities|IsValid (Variables|Default|GetAs%20BP%20Laser%20Sensor)
    (:Is%20Valid
      (Variables|/Game/Item_System/Item/BP_LaserSensor.BP_LaserSensor_C|SetRed (Variables|Default|GetAs%20BP%20Laser%20Sensor) false)
      (Utilities|Array|RemoveItem (Variables|/Game/Item_System/Item/BP_LaserSensor.BP_LaserSensor_C|GetRedLaser (Variables|Default|GetAs%20BP%20Laser%20Sensor)) self))
    (:Is%20Not%20Valid
      _))
  (while (LocalVariables|GetL_Continue)
    (Utilities|FlowControl|Sequence
      (:then_0
        (bind (_outhit _returnvalue) (Collision|LineTraceByChannel (LocalVariables|GetL_CastOrigin) (+ (LocalVariables|GetL_CastOrigin) (* (LocalVariables|GetL_CastDirection) (LocalVariables|GetL_CastDistance))) "TraceTypeQuery3" true 0 "None" true "(R=0.806596,G=1.000000,B=0.000000,A=1.000000)" "(R=0.000000,G=1.000000,B=0.000000,A=1.000000)" 0.1))
        (LocalVariables|SetL_BeamStart (LocalVariables|GetL_CastOrigin))
        (if _returnvalue
          (LocalVariables|SetL_BeamEnd (.ImpactPoint (Collision|BreakHitResult _outhit)))
          (if (Math|Boolean|ORBoolean (.bSuccess (Utilities|Casting|CastToBP_MirrorCube (.HitActor (Collision|BreakHitResult _outhit)))) (.bSuccess (Utilities|Casting|CastToBP_MirrorPlane (.HitActor (Collision|BreakHitResult _outhit)))) (.bSuccess (Utilities|Casting|CastToBP_MirrorCubeHuge (.HitActor (Collision|BreakHitResult _outhit)))) (.bSuccess (Utilities|Casting|CastToBP_MirrorPlaneSmall (.HitActor (Collision|BreakHitResult _outhit)))))
            (LocalVariables|SetL_CastOrigin (.ImpactPoint (Collision|BreakHitResult _outhit)))
            (LocalVariables|SetL_CastDirection (Math|Vector|MirrorVectorbyNormal (LocalVariables|GetL_CastDirection) (.ImpactNormal (Collision|BreakHitResult _outhit))))
            (LocalVariables|SetL_Continue true)
            (else
              (if (.bSuccess (Utilities|Casting|CastToBP_LaserSensor (.HitActor (Collision|BreakHitResult _outhit)))) :!label _label
                (bind _output_get (Variables|Default|SetAs%20BP%20Laser%20Sensor (.AsBP%20Laser%20Sensor (Utilities|Casting|CastToBP_LaserSensor (.HitActor (Collision|BreakHitResult _outhit))))))
                (Variables|/Game/Item_System/Item/BP_LaserSensor.BP_LaserSensor_C|SetRed _output_get true)
                (Utilities|Array|AddUnique (Variables|/Game/Item_System/Item/BP_LaserSensor.BP_LaserSensor_C|GetRedLaser _output_get) self)
                (LocalVariables|SetL_Continue false)
                (else
                  (LocalVariables|SetL_Continue false)))))
          (else
            (LocalVariables|SetL_BeamEnd (+ (LocalVariables|GetL_CastOrigin) (* (LocalVariables|GetL_CastDirection) (LocalVariables|GetL_CastDistance))))
            (goto _label))))
      (:then_1
        (bind _returnvalue_2 (Game|SpawnActorfromClass "/Game/Blueprints/BP_LightBeamRed.BP_LightBeamRed_C" (Math|Transform|MakeTransform "0, 0, 0" "0, 0, 0" "1.000000,1.000000,1.000000") "Undefined" "MultiplyWithRoot" 0 0))
        (Default|SetEnds _returnvalue_2 (LocalVariables|GetL_BeamStart) (LocalVariables|GetL_BeamEnd))
        (Utilities|Array|Add (Variables|Default|GetBeams) _returnvalue_2)))))