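; BP_LightFan is a fan item that acts as a thruster on the items linked to it while Active.
; Each tick it eases the blade spin toward TargetSpeed when active, or more quickly down to rest when inactive.
; While active, it pushes every attached-to and received item along the fan's right vector, applying force at the fan's location so off-center placement also produces torque.
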(event EventTick
  (params (DeltaSeconds :type Float%20%28single-precision%29))
  (bind _force (Variables|Default|GetForce))
  (bind _rootstaticmesh (Variables|Default|GetRootStaticmesh))
  (bind _returnvalue (Transformation|GetWorldLocation _rootstaticmesh))
  (bind _returnvalue_2 (Math|Vector|GetRightVector _rootstaticmesh))
  (bind _returnvalue_3 (* _returnvalue_2 _force))
  (if (Variables|Default|GetActive)
    (Utilities|FlowControl|Sequence
      (:then_0
        (bind _output_get (Variables|Default|SetCurrentSpeed (Math|Interpolation|FInterpTo (Variables|Default|GetCurrentSpeed) (Variables|Default|GetTargetSpeed) DeltaSeconds 0.5)))
        (Transformation|AddLocalRotation (Variables|Default|GetFan) (Math|Rotator|MakeRotator 0.0 _output_get 0.0) false false))
      (:then_1
        (for _array_element (Variables|Default|GetAllAttachedToItems)
          (Class|PrimitiveComponent|AddForceatLocation (Variables|/Game/Item_System/Item/BP_ItemBase.BP_ItemBase_C|GetStaticMesh _array_element) _returnvalue_3 _returnvalue "None"))
        (for _array_element_2 (Variables|Default|GetAllReceiveItems)
          (Class|PrimitiveComponent|AddForceatLocation (Variables|/Game/Item_System/Item/BP_ItemBase.BP_ItemBase_C|GetStaticMesh _array_element_2) _returnvalue_3 _returnvalue "None"))))
    (else
      (bind _output_get_2 (Variables|Default|SetCurrentSpeed (Math|Interpolation|FInterpTo (Variables|Default|GetCurrentSpeed) 0.0 DeltaSeconds 1.0)))
      (Transformation|AddLocalRotation (Variables|Default|GetFan) (Math|Rotator|MakeRotator 0.0 _output_get_2 0.0) false false))))

(event Collision|EventActorBeginOverlap
  (params (OtherActor :type Actor%20Object%20Reference))
  (|CallParentFunction OtherActor) ; This node is disabled and will not be called.\nDrag off pins to build functionality.
)

(event EventBeginPlay
  (|CallParentFunction) ; This node is disabled and will not be called.\nDrag off pins to build functionality.
)

(fn ConstructionScript
  (|CallParentFunction))