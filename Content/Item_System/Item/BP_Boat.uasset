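; BP_Boat is a physics-driven boat in the item system that other items can be attached to.
; AddMesh extends the parent attach logic, adding buoyancy when the attached item's function is "Float".
; The C key toggles fan thrust, and Tick applies force at each valid fan's location along its up vector.
; High angular damping on the static mesh, set at BeginPlay, resists rotation from these off-center forces.
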(event EventBeginPlay
  (|CallParentFunction)
  (Class|PrimitiveComponent|SetAngularDamping (Variables|Default|GetStaticMesh) 5e+01))

(event Collision|EventActorBeginOverlap
  (params (OtherActor :type Actor%20Object%20Reference))
  (|CallParentFunction OtherActor) ; This node is disabled and will not be called.\nDrag off pins to build functionality.
)

(event EventTick
  (params (DeltaSeconds :type Float%20%28single-precision%29))
  (|CallParentFunction DeltaSeconds)
  (if (Variables|Default|GetActiveFans)
    (for _array_element (Variables|Default|GetFans)
      (Utilities|IsValid _array_element
        (:Is%20Valid
          (Class|PrimitiveComponent|AddForceatLocation (Variables|Default|GetStaticMesh) (* (Math|Vector|GetUpVector _array_element) (Variables|Default|GetForce)) (Transformation|GetWorldLocation _array_element) "None"))))))

(event Input|KeyboardEvents|C
  (params (Key :type Key%20Structure :default "None"))
  (:Pressed
    (Utilities|FlowControl|FlipFlop
      (:A
        (Variables|Default|SetActiveFans true))
      (:B
        (Variables|Default|SetActiveFans false)))))

(fn ConstructionScript
  (|CallParentFunction))

(fn AddMesh
  (params (AnotherItem :type BP%20Item%20Object%20Reference) (PointMain :type Scene%20Component%20Object%20Reference) (Material :type Material%20Interface%20Object%20Reference) (PointGrab :type Scene%20Component%20Object%20Reference))
  (bind (_success _mesh) (|CallParentFunction AnotherItem PointMain Material PointGrab))
  (if (Utilities|Enum|Equal(Enum) (Variables|/Game/Item_System/Item/BP_ItemBase.BP_ItemBase_C|GetFunction AnotherItem) "Float")
    (AddComponent|AddBuoyancyComponent self))
  (return _success _mesh))