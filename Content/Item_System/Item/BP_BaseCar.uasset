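; Base car item in the combinable item system, driven by physics through attached parts and steering input.
; While controllable with a forward wheel, Tick applies yaw torque to the root mesh from the negated RotWheel value.
; ActiveFan pushes the mesh at each attached "Accelerate" item along that item's up vector.
; Combine only calls the parent; its front-wheel detection that sets HaveForwardWheel is disconnected.
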(event Custom|RotWheel
  (params (Value :type Float%20%28single-precision%29))
  (Variables|Default|SetRotValue (* Value -1.0)))

(event EventBeginPlay
  (|CallParentFunction))

(event EventTick
  (params (DeltaSeconds :type Float%20%28single-precision%29))
  (|CallParentFunction DeltaSeconds)
  (Utilities|FlowControl|Sequence
    (:then_1
      (if (Variables|Default|GetCanControl)
        (if (Variables|Default|GetHaveForwardWheel)
          (Class|PrimitiveComponent|AddTorqueinRadians (Variables|Default|GetRootStaticmesh) (Math|Vector|MakeVector 0.0 0.0 (* (Variables|Default|GetRotValue) 1e+01)) "None" true))))))

(fn ConstructionScript
  (|CallParentFunction))

(fn Combine
  (params (AnotherItem :type BP%20Item%20Object%20Reference) (PointMain :type Scene%20Component%20Object%20Reference) (PointGrab :type Scene%20Component%20Object%20Reference))
  (|CallParentFunction AnotherItem PointMain PointGrab))

(fn ActiveFan
  (if true
    (for _array_element (Variables|Default|GetAllReceiveItems)
      (if (Utilities|Enum|Equal(Enum) (Variables|/Game/Item_System/Item/BP_ItemBase.BP_ItemBase_C|GetFunction _array_element) "Accelerate")
        (Class|PrimitiveComponent|AddForceatLocation (Variables|Default|GetStaticMesh) (* (Math|Vector|GetUpVector (Variables|/Script/Engine.Actor|GetRootComponent _array_element)) (Variables|Default|GetForce)) (Transformation|GetWorldLocation (Variables|/Script/Engine.Actor|GetRootComponent _array_element)) "None")))))