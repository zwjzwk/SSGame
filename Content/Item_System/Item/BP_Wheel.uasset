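; BP_Wheel is a physics-driven wheel item that responds to control input with angular impulses on its mesh.
; On control, X input turns it about the controller's up axis, scaled by the wheel's forward offset from that controller.
; Y input spins it about the right axis, using a torque curve over local spin speed and scaled by the main actor's mass.
; An Intensity factor scales the combined impulse.
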(event Custom|OnControl
  (params (Axis :type Vector%202D%20Structure) (ControlActor :type BP%20Control%20Object%20Reference) (MainActor :type BP%20Item%20Base%20Object%20Reference))
  (bind (_x _y) (Math|Vector2D|BreakVector2D Axis))
  (bind _positionpoint (Variables|/Game/Item_System/Item/BP_Control.BP_Control_C|GetPositionPoint ControlActor))
  (Class|PrimitiveComponent|AddAngularImpulseinRadians (Variables|Default|GetStaticMesh) (* (+ (* (* (Math|Vector|GetUpVector _positionpoint) (* _x 233.0 (.X (Math|Vector|BreakVector (.location (Math|Transform|MakeRelativeTransform (Transformation|GetActorTransform) (Transformation|GetWorldTransform _positionpoint))))))) 1.0) (* (* (Math|Vector|GetRightVector _positionpoint) (* _y (* (Math|Curves|GetFloatValue (Variables|Default|GetTouqueCurve_ControlStick) (CallFunction|WheelRotateSpeed)) -1.0 0.25))) (/ (Physics|GetMass (Variables|/Game/Item_System/Item/BP_ItemBase.BP_ItemBase_C|GetRootStaticmesh MainActor)) 2e+01))) (Variables|Default|GetIntensity)) "None" false))

(event EventBeginPlay
  (|CallParentFunction) ; This node is disabled and will not be called.\nDrag off pins to build functionality.
)

(event Collision|EventActorBeginOverlap
  (params (OtherActor :type Actor%20Object%20Reference))
  (|CallParentFunction OtherActor) ; This node is disabled and will not be called.\nDrag off pins to build functionality.
)

(event EventTick
  (params (DeltaSeconds :type Float%20%28single-precision%29))
  (|CallParentFunction DeltaSeconds))

(fn ConstructionScript
  (|CallParentFunction))

(fn WheelRotateSpeed
  (bind _staticmesh (Variables|Default|GetStaticMesh))
  (return (.X (Math|Vector|BreakVector (Math|Transform|InverseTransformDirection (Transformation|GetWorldTransform _staticmesh) (Physics|GetPhysicsAngularVelocityinDegrees _staticmesh "None"))))))