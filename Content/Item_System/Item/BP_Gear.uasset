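; BP_Gear is a gear item that spins while Active, built on a parent class whose Tick it calls first.
; Each active tick adds a fixed local rotation to the root mesh without delta-time scaling, so spin speed follows frame rate.
; Physics simulation turns off while active with both receive and attached-to item lists non-empty, and back on whenever inactive.
; An unconnected torque-based spin remains unused.
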(event EventBeginPlay
  (|CallParentFunction) ; This node is disabled and will not be called.\nDrag off pins to build functionality.
)

(event Collision|EventActorBeginOverlap
  (params (OtherActor :type Actor%20Object%20Reference))
  (|CallParentFunction OtherActor) ; This node is disabled and will not be called.\nDrag off pins to build functionality.
)

(event EventTick
  (params (DeltaSeconds :type Float%20%28single-precision%29))
  (|CallParentFunction DeltaSeconds)
  (if (Variables|Default|GetActive)
    (Utilities|FlowControl|Sequence
      (:then_0
        (Transformation|AddLocalRotation (Variables|Default|GetRootStaticmesh) "0,7.000000, 0" false false))
      (:then_1
        (if (and (!= (Utilities|Array|Length (Variables|Default|GetAllReceiveItems)) 0) (!= (Utilities|Array|Length (Variables|Default|GetAllAttachedToItems)) 0))
          (Physics|SetSimulatePhysics (Variables|Default|GetRootStaticmesh) false))))
    (else
      (Physics|SetSimulatePhysics (Variables|Default|GetRootStaticmesh) true))))

(fn ConstructionScript
  (|CallParentFunction))