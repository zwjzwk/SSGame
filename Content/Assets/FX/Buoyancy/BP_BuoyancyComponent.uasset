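; Actor component that floats a physics-simulated primitive on water, using pontoon points supplied by the owner through a buoyancy interface.
; An attached Niagara system spawns one particle per pontoon and exports water height and normal back to the component.
; Each tick applies damped buoyancy from submerged sphere volume, plus linear and angular drag, at each pontoon.
; An optional first-update snap aligns the mesh to a best-fit plane found by gradient descent.
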(event EventParticleData
  (params (Data :type Array%20of%20Basic%20Particle%20Data%20Structures) (NiagaraSystem :type Niagara%20System%20Object%20Reference))
  (Variables|Buoyancy|SetReadbackData Data))

(event EventBeginPlay
  (if (Variables|Settings|GetbActivateUponStart)
    (Buoyancy|Pontoon|EnableBuoyancy false)))

(event EventEndPlay
  (params (EndPlayReason :type EEndPlayReason%20Enum :default "Destroyed"))
  (Buoyancy|Pontoon|DisableBuoyancy))

(event EventTick
  (params (DeltaSeconds :type Float%20%28single-precision%29))
  (if (Components|Activation|IsActive)
    (Buoyancy|Pontoon|UpdateBuoyancy)))

(fn InitiateBuoyancy
  (bind _readbackdata (Variables|Buoyancy|GetReadbackData))
  (bind _buoyantprimitive (Variables|Default|GetBuoyantPrimitive))
  (Utilities|IsValid _buoyantprimitive
    (:Is%20Valid
      (LocalVariables|SetThisBuoyantPrimitiveTransform (Transformation|GetWorldTransform _buoyantprimitive))
      (LocalVariables|SetThisBuoyantPrimitiveScale (Transformation|GetWorldScale _buoyantprimitive))
      ;[1 1 1] build list of pontoons positions projected on the water surface
      (for (_array_element _array_index) (Variables|Buoyancy|GetPontoons)
        (if (Utilities|Array|IsValidIndex _readbackdata _array_index)
          (Utilities|Array|Add (LocalVariables|GetThoseBuoyantDataPositions) (Math|Vector|MakeVector (.X (Math|Vector|BreakVector (Math|Transform|TransformLocation (LocalVariables|GetThisBuoyantPrimitiveTransform) (/ _array_element (LocalVariables|GetThisBuoyantPrimitiveScale))))) (.Y (Math|Vector|BreakVector (Math|Transform|TransformLocation (LocalVariables|GetThisBuoyantPrimitiveTransform) (/ _array_element (LocalVariables|GetThisBuoyantPrimitiveScale))))) (.Size (Utilities|Struct|BreakBasicParticleData (Utilities|Array|Get(acopy) _readbackdata _array_index)))))
          (else
            (return false))))
      ;[1 1 1] initiate buoyant mesh's location & rotation to somewhat match the water surface. Don't actually simulate buoyancy. This just ensures the buoyant mesh is somewhat adequatelly positioned & rotated so buoyancy simulation is somewhat neutral from the get go (meaning the mesh is somewhat floating already and nothing crazy happens). This isn't perfect and is quite costly in BP.
      (bind (_location _normal) (Buoyancy|Initiate|GetBestFittingPlanefromPoints (LocalVariables|GetThoseBuoyantDataPositions) 1e-05 0.0001))
      (Transformation|SetWorldLocationAndRotation (Variables|Default|GetBuoyantPrimitive) _location (Math|Rotator|MakeRotationfromAxes (Math|Vector|CrossProduct (Math|Vector|CrossProduct _normal (Math|Vector|GetForwardVector (Variables|Default|GetBuoyantPrimitive))) _normal) (Math|Vector|CrossProduct _normal (Math|Vector|GetForwardVector (Variables|Default|GetBuoyantPrimitive))) _normal) true true)
      (return true))
    (:Is%20Not%20Valid
      (return false))))

(fn GetBestFittingPlaneScore
  (params (Vectors :type Array%20of%20Vectors) (Location :type Vector) (Normal :type Vector))
  (for _array_element Vectors
    (bind _output_get (LocalVariables|SetThisPlanarDistance (Math|Float|Absolute(Float) (Math|Vector|DotProduct (- _array_element Location) Normal))))
    (LocalVariables|SetThisSumOfSquared (+ (Math|Float|Square _output_get) (LocalVariables|GetThisSumOfSquared))))
  (return (LocalVariables|GetThisSumOfSquared)))

(fn GetBestFittingPlanefromPoints
  (params (Vectors :type Array%20of%20Vectors) (DerivativeStep :type Float%20%28single-precision%29) (Step :type Float%20%28single-precision%29))
  ;[1 1 1] initiate plane location/normal. We only really need to perform an iterative search for the plane's normal
  (LocalVariables|SetThisLocation (Math|Vector|GetVectorArrayAverage Vectors))
  (LocalVariables|SetThoseNormalComponents (Utilities|Array|MakeArray 0.0 0.0 1.0))
  (LocalVariables|SetThisNormal "0, 0,1.000000")
  ;[1 1 1] iterative algorithm. Ideally you'd early exit if you get a gradient magnitude close enough to 0 but I skipped it for simplicity sake
  (for _index (range 0 (- (Variables|Settings|Snap|GetSnapToWaterIterations) 1))
    ;[1 1 1] for each normal's XYZ component
    (for (_array_element _array_index) (LocalVariables|GetThoseNormalComponents)
      (LocalVariables|SetThisComponentValue _array_element)
      (LocalVariables|SetThisComponentIndex _array_index)
      ;[1 1 1] get score with components as-is
      (bind _sumofsquared (Buoyancy|Initiate|GetBestFittingPlaneScore Vectors (LocalVariables|GetThisLocation) (LocalVariables|GetThisNormal)))
      (LocalVariables|SetThisScore1 _sumofsquared)
      ;[1 1 1] nudge component ever so slightly and get new score
      (bind _sumofsquared_2 (Buoyancy|Initiate|GetBestFittingPlaneScore Vectors (LocalVariables|GetThisLocation) (Math|Vector|Normalize (+ (LocalVariables|GetThisNormal) (* (Utilities|Select :Index (LocalVariables|GetThisComponentIndex) :Option%200 "1.000000, 0, 0" :Option%201 "0,1.000000, 0" :Option%202 "0, 0,1.000000") DerivativeStep)))))
      (LocalVariables|SetThisScore2 _sumofsquared_2)
      ;[1 1 1] derive gradient from two scores and nudge normal component towards that gradient for next iteration
      (Utilities|Array|SetArrayElem (LocalVariables|GetThoseNormalComponents) (LocalVariables|GetThisComponentIndex) (+ (LocalVariables|GetThisComponentValue) (* Step (/ (- (LocalVariables|GetThisScore1) (LocalVariables|GetThisScore2)) DerivativeStep)))))
    (LocalVariables|SetThisNormal (Math|Vector|Normalize (Math|Vector|MakeVector (Utilities|Array|Get(acopy) (LocalVariables|GetThoseNormalComponents)) (Utilities|Array|Get(acopy) (LocalVariables|GetThoseNormalComponents) 1) (Utilities|Array|Get(acopy) (LocalVariables|GetThoseNormalComponents) 2)))))
  (return (LocalVariables|GetThisLocation) (LocalVariables|GetThisNormal)))

(fn EnableBuoyancy
  (params (bForceSnapToWater :type Boolean))
  (bind _returnvalue (Components|GetOwner))
  ;[1 1 1] component must NOT be already active. Then readback system must be specified by user, then owner must be valid and implement our buoyancy interface
  (if (not (Components|Activation|IsActive))
    (Utilities|IsValid (Variables|Settings|GetSystem)
      (:Is%20Valid
        (Utilities|IsValid _returnvalue
          (:Is%20Valid
            (if (Utilities|DoesObjectImplementInterface _returnvalue "/Game/Assets/FX/Buoyancy/BPI_BuoyancySystem_Interface.BPI_BuoyancySystem_Interface_C")
              ;[1 1 1] ask actor where to attach Niagara readback system via buoyancy interface (and make sure that primitive does simulate physics)
              (bind _primitivecomponent (Class|BPIBuoyancySystemInterface|GetBuoyancyPrimitive(Message) (Components|GetOwner)))
              (Utilities|IsValid _primitivecomponent
                (:Is%20Valid
                  (bind _output_get (Variables|Default|SetBuoyantPrimitive _primitivecomponent))
                  (Physics|SetSimulatePhysics _output_get true)
                  ;[1 1 1] ask actor its buoyant points (what's usually referred as 'pontoons') and cache them here to ensure those stay the same for the duration of the buoyancy
                  (bind _pontoons (Class|BPIBuoyancySystemInterface|GetBuoyancyPontoons(Message) (Components|GetOwner)))
                  (if (> (Utilities|Array|Length _pontoons) 0)
                    (Variables|Buoyancy|SetPontoons _pontoons)
                    (Utilities|FlowControl|Sequence
                      (:then_0
                        ;[1 1 1] start with a clean slate
                        (Utilities|Array|Clear (Variables|Buoyancy|GetReadbackData))
                        (Utilities|Array|Clear (Variables|Buoyancy|GetPontoonsDepth))
                        (Utilities|Array|Clear (Variables|Buoyancy|GetPontoonsPreviousLocations)))
                      (:then_1
                        ;[1 1 1] Niagara system might have persisted through a previous 'DisableBuoyancy' call (might not have been destroyed by user), in that case we paused it! So unpause it. Else create & attach it!
                        (Utilities|IsValid (Variables|Default|GetReadbackSystem)
                          (:Is%20Valid
                            (if (== (Transformation|GetAttachParent (Variables|Default|GetReadbackSystem)) (Variables|Default|GetBuoyantPrimitive)) ; Just make sure it's still correctly attached to that same primitive
                              (Class|NiagaraComponent|SetPaused (Variables|Default|GetReadbackSystem) false)
                              (else
                                (bind _returnvalue_2 (Niagara|SpawnSystemAttached (Variables|Settings|GetSystem) (Variables|Default|GetBuoyantPrimitive) "None" "0, 0, 0" "0, 0, 0" "SnapToTargetIncludingScale" false true "None" false :!label _label))
                                (Variables|Default|SetReadbackSystem _returnvalue_2))))
                          (:Is%20Not%20Valid
                            (goto _label)))
                        ;[1 1 1] spawn one particle per pontoon
                        (Class|NiagaraDataInterfaceArrayFunctionLibrary|SetNiagaraArrayVector (Variables|Default|GetReadbackSystem) "Pontoons" (Variables|Buoyancy|GetPontoons))
                        ;[1 1 1] Niagara readback system will report back to us
                        (Class|NiagaraComponent|SetVariableObject (Variables|Default|GetReadbackSystem) "Blueprint" self)
                        ;[1 1 1] reinitialize system to make sure the correct amount of particles are spawned (one per 'pontoon')
                        (Niagara|ReinitializeSystem (Variables|Default|GetReadbackSystem))
                        ;[1 1 1] enable exporter interface!
                        (Class|NiagaraComponent|SetVariableBool (Variables|Default|GetReadbackSystem) "bExportBuoyancy" true)
                        (Variables|Buoyancy|SetbSnapToWaterRequested (or (Variables|Settings|Snap|GetbSnapToWaterOnActivation) bForceSnapToWater))
                        ;[1 1 1] buoyancy has started! broadcast message (and send Niagara readback system along the way, why not, might be useful)
                        (Components|Activation|Activate false)
                        (Components|Tick|SetComponentTickEnabled true)
                        (Default|CallBuoyancyStarted (Variables|Default|GetReadbackSystem))
                        (return true)))
                    (else
                      (return false))))
                (:Is%20Not%20Valid
                  (return false)))))
          (:Is%20Not%20Valid
            (return false))))
      (:Is%20Not%20Valid
        (return false)))
    (else
      (return false))))

(fn DisableBuoyancy
  (bind _buoyantprimitive (Variables|Default|GetBuoyantPrimitive))
  (bind _readbacksystem (Variables|Default|GetReadbackSystem))
  ;[1 1 1] disable only if it was enabled in the first place! Then broadcast message. User might want to destroy the Niagara readback emitter upon receiving this message ('DestroyComponent' can only be called by the actor actually owning it, so... not us)
  (if (Components|Activation|IsActive)
    (Components|Activation|Deactivate)
    (Default|CallBuoyancyStopped _readbacksystem)
    (Utilities|FlowControl|Sequence
      (:then_0
        (Utilities|IsValid _readbacksystem
          (:Is%20Valid
            ;[1 1 1] if user chose NOT to destroy Niagara readback emitter, we might be able to re use it next time Buoyancy is activated, so for now pause it and disable exporter interface
            (Class|NiagaraComponent|SetPaused _readbacksystem true)
            (Class|NiagaraComponent|SetVariableBool _readbacksystem "bExportBuoyancy" false))))
      (:then_1
        (Utilities|IsValid _buoyantprimitive
          (:Is%20Valid
            (Physics|SetSimulatePhysics _buoyantprimitive false) ; freeze primitive in place
          )))
      (:then_2
        (Components|Tick|SetComponentTickEnabled false)
        (return true)))
    (else
      (return false))))

(fn ApplyBuoyancy
  (bind _buoyantprimitive (Variables|Default|GetBuoyantPrimitive))
  (bind _radius (Variables|Settings|GetRadius))
  (bind _buoyantprimitive_2 (Variables|Default|GetBuoyantPrimitive))
  (bind _pontoonspreviouslocations (Variables|Buoyancy|GetPontoonsPreviousLocations))
  (bind _maxdragspeed (Variables|Settings|Drag|Linear|GetMaxDragSpeed))
  (bind _pontoons (Variables|Buoyancy|GetPontoons))
  (bind _returnvalue (* _radius 2.0))
  ;[1 1 1] ensure everything is good to go & cache buoyant primitive's transform
  (Utilities|IsValid _buoyantprimitive_2
    (:Is%20Valid
      (if (Physics|IsSimulatingPhysics _buoyantprimitive_2 "None")
        (LocalVariables|SetThisBuoyantPrimitiveTransform (Transformation|GetWorldTransform _buoyantprimitive_2))
        (LocalVariables|SetThisBuyoantPrimitiveScale (Transformation|GetWorldScale _buoyantprimitive_2))
        ;[1 1 1] for each pontoon, get pontoon's location in world space
        (LocalVariables|SetThisPontoonCount (Math|Conversions|ToFloat(Integer) (Utilities|Array|Length _pontoons)))
        (for (_array_element _array_index) _pontoons
          (bind _output_get (LocalVariables|SetThisPontoonIndex _array_index))
          (if (Utilities|Array|IsValidIndex (Variables|Buoyancy|GetReadbackData) _output_get) ; ensure readback data is valid
            (LocalVariables|SetThisPontoonLocation (Math|Transform|TransformLocation (LocalVariables|GetThisBuoyantPrimitiveTransform) (/ _array_element (LocalVariables|GetThisBuyoantPrimitiveScale))))
            ;[1 1 1] get pontoon's velocity in world space based on its previous position (if any) and replace its previous position with current one
            (if (Utilities|Array|IsValidIndex _pontoonspreviouslocations (LocalVariables|GetThisPontoonIndex))
              (LocalVariables|SetThisPontoonVelocity (/ (- (LocalVariables|GetThisPontoonLocation) (Utilities|Array|Get(acopy) _pontoonspreviouslocations (LocalVariables|GetThisPontoonIndex))) (Utilities|Time|GetWorldDeltaSeconds)))
              (else
                (LocalVariables|SetThisPontoonVelocity "0, 0, 0")))
            (Utilities|Array|SetArrayElem (Variables|Buoyancy|GetPontoonsPreviousLocations) (LocalVariables|GetThisPontoonIndex) (LocalVariables|GetThisPontoonLocation) true)
            ;[1 1 1] get readback data at that pontoon index and compute depth based on pontoon's sphere radius and water level
            (bind _output_get_2 (LocalVariables|SetThisReadbackData (Utilities|Array|Get(acopy) (Variables|Buoyancy|GetReadbackData) (LocalVariables|GetThisPontoonIndex))))
            (LocalVariables|SetThisPontoonVerticalDistance (+ (- (.Size (Utilities|Struct|BreakBasicParticleData _output_get_2)) (.Z (Math|Vector|BreakVector (LocalVariables|GetThisPontoonLocation)))) (Variables|Settings|GetOffset) _radius))
            (Utilities|Array|SetArrayElem (Variables|Buoyancy|GetPontoonsDepth) (LocalVariables|GetThisPontoonIndex) (LocalVariables|GetThisPontoonVerticalDistance) true)
            (bind _output_get_3 (LocalVariables|SetThisPontoonDepth (Math|Float|Clamp(Float) (LocalVariables|GetThisPontoonVerticalDistance) 0.0 _returnvalue)))
            (if (> _output_get_3 0.0)
              (LocalVariables|SetThisPontoonNormalizedDepth (/ _output_get_3 _returnvalue))
              ;[1 1 1] get this pontoon's submerged volume (sphere partial volume equation from height is 1/3 * PI * H^2 * (3R - H)). That's how much fluid is displaced with is the main factor to compute buoyancy force (fluid density is skipped)
              (LocalVariables|SetThisSubmergedVolume (* (Math|Float|MultiplybyPi 0.333333) (Math|Float|Square (LocalVariables|GetThisPontoonDepth)) (- (* 3.0 (Variables|Settings|GetRadius)) (LocalVariables|GetThisPontoonDepth))))
              ;[1 1 1] compute a vertical damping force. Damping vertical force is an important part of buoyancy
              (LocalVariables|SetThisDamp (Math|Float|Max(Float) (+ (* (Variables|Settings|Damping|GetDampingFactor1) (.Z (Math|Vector|BreakVector (LocalVariables|GetThisPontoonVelocity)))) (* (Math|Float|Sign(Float) (.Z (Math|Vector|BreakVector (LocalVariables|GetThisPontoonVelocity)))) (Math|Float|Square (.Z (Math|Vector|BreakVector (LocalVariables|GetThisPontoonVelocity)))) (Variables|Settings|Damping|GetDampingFactor2))) 0.0))
              ;[1 1 1] apply buoyancy force
              (bind _output_get_4 (LocalVariables|SetThisForce (* (Math|Vector|Lerp(Vector) "0, 0,1.000000" (.Velocity (Utilities|Struct|BreakBasicParticleData (LocalVariables|GetThisReadbackData))) (Variables|Settings|GetApplyWaveNormal)) (* (Math|Float|Clamp(Float) (- (LocalVariables|GetThisSubmergedVolume) (LocalVariables|GetThisDamp)) 0.0 (Variables|Settings|Force|GetMaxForce)) (Variables|Settings|Force|GetCoefficient)))))
              (Class|PrimitiveComponent|AddForceatLocation (Variables|Default|GetBuoyantPrimitive) _output_get_4 (LocalVariables|GetThisPontoonLocation) "None")
              (Utilities|FlowControl|Sequence
                (:then_0
                  ;[1 0.1 0] draw debug (to remove)
                  (if (Variables|Settings|Debug|GetbDrawDebug)
                    (Rendering|Debug|DrawDebugLine (LocalVariables|GetThisPontoonLocation) (+ (LocalVariables|GetThisPontoonLocation) (* (LocalVariables|GetThisForce) 0.0025)) "(R=1.000000,G=0.250158,B=0.000000,A=1.000000)" 0.0 6.0)
                    (Rendering|Debug|DrawDebugSphere (LocalVariables|GetThisPontoonLocation) (Variables|Settings|GetRadius) 12 "(R=1.000000,G=0.250158,B=0.000000,A=1.000000)" 0.0 2.0)))
                (:then_1
                  ;[1 1 1] apply linear drag if pontoon is in water & moving in planar space at all
                  (if (or (> (Variables|Settings|Drag|Linear|GetDragCoefficient) 0.0) (> (Variables|Settings|Drag|Linear|GetDragCoefficient2) 0.0))
                    (bind _output_get_5 (LocalVariables|SetThisPontoonVelocityInKmh (* (LocalVariables|GetThisPontoonVelocity) "0.036000,0.036000,0.000000")))
                    (bind _output_get_6 (LocalVariables|SetThisPontoonSpeedInKmh (Math|Vector|VectorLength _output_get_5)))
                    (if (> _output_get_6 0.0001)
                      (bind _output_get_7 (LocalVariables|SetThisPontoonClampedSpeedInKmh (Math|Float|Clamp(Float) _output_get_6 (* _maxdragspeed -1.0) _maxdragspeed)))
                      (LocalVariables|SetThisPontoonMovementDirection (/ (LocalVariables|GetThisPontoonVelocityInKmh) _output_get_7))
                      ;[1 1 1] compute linear drag force
                      (Utilities|FlowControl|Sequence
                        (:then_0
                          (LocalVariables|SetThisForce (* (LocalVariables|GetThisPontoonMovementDirection) (* (* (LocalVariables|GetThisPontoonClampedSpeedInKmh) (Variables|Settings|Drag|Linear|GetDragCoefficient)) -1.0))))
                        (:then_1
                          (LocalVariables|SetThisForce (- (LocalVariables|GetThisForce) (* (LocalVariables|GetThisPontoonMovementDirection) (* (* (LocalVariables|GetThisPontoonClampedSpeedInKmh) (LocalVariables|GetThisPontoonClampedSpeedInKmh) (Variables|Settings|Drag|Linear|GetDragCoefficient2)) (LocalVariables|GetThisPontoonSpeedInKmh))))))
                        (:then_2
                          (Class|PrimitiveComponent|AddForceatLocation (Variables|Default|GetBuoyantPrimitive) (LocalVariables|GetThisForce) (LocalVariables|GetThisPontoonLocation) "None"))))))
                (:then_2
                  ;[1 1 1] apply angular drag if pontoon is in water
                  (if (> (Variables|Settings|Drag|Angular|GetAngularDrag) 0.0)
                    (Class|PrimitiveComponent|AddTorqueinRadians _buoyantprimitive (* (Class|PrimitiveComponent|GetPhysicsAngularVelocityinRadians _buoyantprimitive "None") (* -1.0 (/ (Variables|Settings|Drag|Angular|GetAngularDrag) (LocalVariables|GetThisPontoonCount)))) "None" false)))))))
        (else
          (return false))))
    (:Is%20Not%20Valid
      (return false))))

(fn UpdateBuoyancy
  ;[1 1 1] we might want to project mesh onto water surface the very first update. Only process actual buoyancy next update, after projection was processed (if only projection was requested!)
  (if (Variables|Buoyancy|GetbSnapToWaterRequested)
    (bind _binitiated (Buoyancy|Initiate|InitiateBuoyancy))
    (if _binitiated
      (Variables|Buoyancy|SetbSnapToWaterRequested false) ; consume
      (else
        (return false)))
    (else
      (Buoyancy|Pontoon|ApplyBuoyancy)))
  (Default|CallBuoyancyApplied) ; broadcast event to actor
  (return true))