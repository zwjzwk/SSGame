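; Plug actor, apparently a puzzle piece, that turns on a laser when linked to another plug with at least five cubes present.
; Box overlaps with another BP_Plug set the Connect flag, while Box1 overlaps keep a running count of BP_SimpleCube actors.
; Tick checks both conditions to toggle the laser and manually advances the Niagara simulation by twice the frame time.
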(event OnComponentBeginOverlap(Box)
  (params (OverlappedComponent :type Primitive%20Component%20Object%20Reference) (OtherActor :type Actor%20Object%20Reference) (OtherComp :type Primitive%20Component%20Object%20Reference) (OtherBodyIndex :type Integer) (bFromSweep :type Boolean) (SweepResult :type Hit%20Result%20Structure%20%28by%20ref%29))
  (Utilities|Casting|CastToBP_Plug OtherActor)
  (Variables|Default|SetConnect true))

(event OnComponentEndOverlap(Box)
  (params (OverlappedComponent :type Primitive%20Component%20Object%20Reference) (OtherActor :type Actor%20Object%20Reference) (OtherComp :type Primitive%20Component%20Object%20Reference) (OtherBodyIndex :type Integer))
  (Utilities|Casting|CastToBP_Plug OtherActor)
  (Variables|Default|SetConnect false))

(event OnComponentBeginOverlap(Box1)
  (params (OverlappedComponent :type Primitive%20Component%20Object%20Reference) (OtherActor :type Actor%20Object%20Reference) (OtherComp :type Primitive%20Component%20Object%20Reference) (OtherBodyIndex :type Integer) (bFromSweep :type Boolean) (SweepResult :type Hit%20Result%20Structure%20%28by%20ref%29))
  (Utilities|Casting|CastToBP_SimpleCube OtherActor)
  (Variables|Default|SetCubeNums (+ (Variables|Default|GetCubeNums) 1)))

(event OnComponentEndOverlap(Box1)
  (params (OverlappedComponent :type Primitive%20Component%20Object%20Reference) (OtherActor :type Actor%20Object%20Reference) (OtherComp :type Primitive%20Component%20Object%20Reference) (OtherBodyIndex :type Integer))
  (Utilities|Casting|CastToBP_SimpleCube OtherActor)
  (Variables|Default|SetCubeNums (- (Variables|Default|GetCubeNums) 1)))

(event EventBeginPlay
  (|CallParentFunction) ; This node is disabled and will not be called.\nDrag off pins to build functionality.
)

(event Collision|EventActorBeginOverlap
  (params (OtherActor :type Actor%20Object%20Reference))
  (|CallParentFunction OtherActor) ; This node is disabled and will not be called.\nDrag off pins to build functionality.
)

(event EventTick
  (params (DeltaSeconds :type Float%20%28single-precision%29))
  (bind _laser (Variables|Default|GetLaser))
  (|CallParentFunction DeltaSeconds)
  (Class|NiagaraComponent|AdvanceSimulation (Variables|Default|GetNiagara) 1 (* DeltaSeconds 2.0))
  (if (and (Variables|Default|GetConnect) (>= (Variables|Default|GetCubeNums) 5))
    (Variables|/Game/Item_System/Item/BP_LaserEmitter.BP_LaserEmitter_C|SetActive _laser true)
    (else
      (Variables|/Game/Item_System/Item/BP_LaserEmitter.BP_LaserEmitter_C|SetActive _laser false))))

(fn ConstructionScript
  (|CallParentFunction))