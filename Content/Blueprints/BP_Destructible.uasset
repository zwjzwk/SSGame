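; A destructible prop that breaks when struck by a fast-moving item or a moving swing.
; The Destructible component's hit event checks the speed of a BP_Item against a threshold, or accepts any movement of a BP_Swing's board.
; A qualifying hit applies tiny-radius damage at the Destructible's location, turns on StaticMesh physics simulation and prints a debug string.
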(event OnComponentHit(Destructible)
  (params (HitComponent :type Primitive%20Component%20Object%20Reference) (OtherActor :type Actor%20Object%20Reference) (OtherComp :type Primitive%20Component%20Object%20Reference) (NormalImpulse :type Vector :default "0, 0, 0") (Hit :type Hit%20Result%20Structure%20%28by%20ref%29))
  (bind _destructible (Variables|Default|GetDestructible))
  (bind _asbp_item (Utilities|Casting|CastToBP_Item OtherActor)
    (:then
      (if (> (Math|Vector|VectorLength (Transformation|GetVelocity _asbp_item)) 1e+03)
        (Class|DestructibleComponent|ApplyRadiusDamage _destructible 1e+02 (Transformation|GetWorldLocation _destructible) 1.0 1.0 true :!label _label)
        (Physics|SetSimulatePhysics (Variables|Default|GetStaticMesh) true)
        (Development|PrintString "Hello")))
    (:CastFailed
      (bind _asbp_swing (Utilities|Casting|CastToBP_Swing OtherActor))
      (if (> (Math|Vector|VectorLength (Transformation|GetComponentVelocity (Variables|/Game/Blueprints/BP_Swing.BP_Swing_C|GetBoard _asbp_swing))) 0.0)
        (goto _label)))))

(event EventBeginPlay)

(event Collision|EventActorBeginOverlap
  (params (OtherActor :type Actor%20Object%20Reference)))

(event EventTick
  (params (DeltaSeconds :type Float%20%28single-precision%29)))

(fn ConstructionScript)