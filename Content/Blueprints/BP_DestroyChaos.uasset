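; BP_DestroyChaos is a destructible prop built on a Chaos geometry collection, with a trigger box that detects impacts from items.
; BeginPlay applies a material to the collection's second material slot.
; An overlapping BP_Item moving above a speed threshold sets the Break flag, provided the player's Magnesis component is not grabbing.
; Nothing here reads Break, and the frame-material and collision-disabling nodes are disconnected.
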(event OnComponentBeginOverlap(Box)
  (params (OverlappedComponent :type Primitive%20Component%20Object%20Reference) (OtherActor :type Actor%20Object%20Reference) (OtherComp :type Primitive%20Component%20Object%20Reference) (OtherBodyIndex :type Integer) (bFromSweep :type Boolean) (SweepResult :type Hit%20Result%20Structure%20%28by%20ref%29))
  (bind _asbp_item (Utilities|Casting|CastToBP_Item OtherActor))
  (bind _asbp_player (Utilities|Casting|CastToBP_Player (Game|Player|GetPlayerPawn 0)))
  (if (and (> (Math|Vector|VectorLength (Transformation|GetVelocity _asbp_item)) 3e+02) (not (Variables|/Game/Item_System/BP_MagnesisComponent.BP_MagnesisComponent_C|GetIsGrabbing (Variables|/Game/ThirdPersonCPP/Blueprints/BP_Player.BP_Player_C|GetBP_MagnesisComponent _asbp_player))))
    (Variables|Default|SetBreak true)))

(event EventBeginPlay
  (Rendering|Material|SetMaterial (Variables|Default|GetCube3_GeometryCollection) 1 "/Game/NewMaterial.NewMaterial"))

(fn ConstructionScript)