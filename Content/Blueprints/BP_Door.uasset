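; BP_Door is a sliding door actor with two parts, R and L, moved by the difference between its Forward and BackWard values.
; Each Tick adds that difference to both parts' local Y offset and accumulates it in Offset.
; Reaching either end of the 0 to 90 travel range sets Stop, after which movement resumes only away from that limit.
; The graph only reads Forward and BackWard, never setting them.
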(event EventBeginPlay)

(event Collision|EventActorBeginOverlap
  (params (OtherActor :type Actor%20Object%20Reference)))

(event EventTick
  (params (DeltaSeconds :type Float%20%28single-precision%29))
  (bind _forward (Variables|Default|GetForward))
  (bind _backward (Variables|Default|GetBackWard))
  (bind _returnvalue (- _forward _backward))
  (if (Math|Boolean|ORBoolean (not (Variables|Default|GetStop)) (and (>= (Variables|Default|GetForward) (Variables|Default|GetBackWard)) (<= (Variables|Default|GetOffset) 0.0)) (and (<= (Variables|Default|GetForward) (Variables|Default|GetBackWard)) (>= (Variables|Default|GetOffset) 9e+01)))
    (Transformation|AddLocalOffset (Variables|Default|GetR) (Math|Vector|MakeVector 0.0 _returnvalue 0.0) false false)
    (Transformation|AddLocalOffset (Variables|Default|GetL) (Math|Vector|MakeVector 0.0 _returnvalue 0.0) false false)
    (bind _output_get (Variables|Default|SetOffset (+ (- (Variables|Default|GetForward) (Variables|Default|GetBackWard)) (Variables|Default|GetOffset))))
    (if (or (>= _output_get 9e+01) (<= _output_get 0.0))
      (Variables|Default|SetStop true)
      (else
        (Variables|Default|SetStop false)))))

(fn ConstructionScript)