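; BP_Slot is a socket actor that detects when a BP_Plug is inserted or removed.
; Its Box overlap events cast the other actor to BP_Plug and react only when the overlapping component is that plug's Plug component.
; Begin and end overlap print on-screen messages reporting connected or disconnected, with no connection state stored.
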(event OnComponentBeginOverlap(Box)
  (params (OverlappedComponent :type Primitive%20Component%20Object%20Reference) (OtherActor :type Actor%20Object%20Reference) (OtherComp :type Primitive%20Component%20Object%20Reference) (OtherBodyIndex :type Integer) (bFromSweep :type Boolean) (SweepResult :type Hit%20Result%20Structure%20%28by%20ref%29))
  (bind _asbp_plug (Utilities|Casting|CastToBP_Plug OtherActor))
  (if (== OtherComp (Variables|/Game/Blueprints/BP_Plug.BP_Plug_C|GetPlug _asbp_plug))
    (Development|PrintString "连通！" true true "(R=0.000000,G=0.660000,B=1.000000,A=1.000000)" 1e+01)))

(event OnComponentEndOverlap(Box)
  (params (OverlappedComponent :type Primitive%20Component%20Object%20Reference) (OtherActor :type Actor%20Object%20Reference) (OtherComp :type Primitive%20Component%20Object%20Reference) (OtherBodyIndex :type Integer))
  (bind _asbp_plug (Utilities|Casting|CastToBP_Plug OtherActor))
  (if (== OtherComp (Variables|/Game/Blueprints/BP_Plug.BP_Plug_C|GetPlug _asbp_plug))
    (Development|PrintString "连接断开！" true true "(R=0.000000,G=0.660000,B=1.000000,A=1.000000)" 1e+01)))

(event EventBeginPlay)

(event Collision|EventActorBeginOverlap
  (params (OtherActor :type Actor%20Object%20Reference)))

(event EventTick
  (params (DeltaSeconds :type Float%20%28single-precision%29)))

(fn ConstructionScript)