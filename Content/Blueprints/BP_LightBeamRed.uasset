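; BP_LightBeamRed is a beam actor, red by its name, that visually connects two world points with a stretched static mesh.
; SetEnds teleports the mesh to the midpoint and aligns its Z axis with the direction between the points.
; It keeps a thin fixed cross-section and scales Z by the distance, assuming a mesh 100 units long.
; The event graph and construction script are empty, so callers drive all placement.
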(event EventBeginPlay)

(event Collision|EventActorBeginOverlap
  (params (OtherActor :type Actor%20Object%20Reference)))

(event EventTick
  (params (DeltaSeconds :type Float%20%28single-precision%29)))

(fn ConstructionScript)

(fn SetEnds
  (params (Begin :type Vector) (End :type Vector))
  (bind _returnvalue (- End Begin))
  (Transformation|SetWorldLocationAndRotation (Variables|Default|GetStaticMesh) (+ Begin (/ _returnvalue 2.0)) (Math|Rotator|MakeRotfromZ (Math|Vector|Normalize _returnvalue)) false true)
  (Transformation|SetWorldScale3D (Variables|Default|GetStaticMesh) (Math|Vector|MakeVector 0.05 0.05 (/ (Math|Vector|VectorLength _returnvalue) 1e+02))))