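; BP_Board is a physics board of three cubes that can link to another board and be cut loose by BP_Cut actors.
; On BeginPlay, enabling Simulate turns physics off on all cubes, and a valid BPBoard reference has its Cube1 and Cube2 constrained to this board's matching cubes.
; Overlaps with BP_Cut break constraints: Cube releases PhysicsConstraint and PhysicsConstraint1, while Cube1 and Cube2 each release their board-to-board link.
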(event OnComponentBeginOverlap(Cube)
  (params (OverlappedComponent :type Primitive%20Component%20Object%20Reference) (OtherActor :type Actor%20Object%20Reference) (OtherComp :type Primitive%20Component%20Object%20Reference) (OtherBodyIndex :type Integer) (bFromSweep :type Boolean) (SweepResult :type Hit%20Result%20Structure%20%28by%20ref%29))
  (Utilities|Casting|CastToBP_Cut OtherActor)
  (Class|PhysicsConstraintComponent|BreakConstraint (Variables|Default|GetPhysicsConstraint))
  (Class|PhysicsConstraintComponent|BreakConstraint (Variables|Default|GetPhysicsConstraint1)))

(event OnComponentBeginOverlap(Cube1)
  (params (OverlappedComponent :type Primitive%20Component%20Object%20Reference) (OtherActor :type Actor%20Object%20Reference) (OtherComp :type Primitive%20Component%20Object%20Reference) (OtherBodyIndex :type Integer) (bFromSweep :type Boolean) (SweepResult :type Hit%20Result%20Structure%20%28by%20ref%29))
  (Utilities|Casting|CastToBP_Cut OtherActor)
  (Class|PhysicsConstraintComponent|BreakConstraint (Variables|Default|GetPhysicsConstraint2)))

(event OnComponentBeginOverlap(Cube2)
  (params (OverlappedComponent :type Primitive%20Component%20Object%20Reference) (OtherActor :type Actor%20Object%20Reference) (OtherComp :type Primitive%20Component%20Object%20Reference) (OtherBodyIndex :type Integer) (bFromSweep :type Boolean) (SweepResult :type Hit%20Result%20Structure%20%28by%20ref%29))
  (Utilities|Casting|CastToBP_Cut OtherActor)
  (Class|PhysicsConstraintComponent|BreakConstraint (Variables|Default|GetPhysicsConstraint3)))

(event EventBeginPlay
  (Utilities|FlowControl|Sequence
    (:then_0
      (if (Variables|Default|GetSimulate)
        (Physics|SetSimulatePhysics (Variables|Default|GetCube1) false)
        (Physics|SetSimulatePhysics (Variables|Default|GetCube) false)
        (Physics|SetSimulatePhysics (Variables|Default|GetCube2) false)))
    (:then_1
      (Utilities|IsValid (Variables|Default|GetBP_Board)
        (:Is%20Valid
          (Class|PhysicsConstraintComponent|SetConstrainedComponents (Variables|Default|GetPhysicsConstraint2) (Variables|Default|GetCube1) "None" (Variables|BP_Board_C|GetCube1 (Variables|Default|GetBP_Board)) "None")
          (Class|PhysicsConstraintComponent|SetConstrainedComponents (Variables|Default|GetPhysicsConstraint3) (Variables|Default|GetCube2) "None" (Variables|BP_Board_C|GetCube2 (Variables|Default|GetBP_Board)) "None"))))))

(fn ConstructionScript)