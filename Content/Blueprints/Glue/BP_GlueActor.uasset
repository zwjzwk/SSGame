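; Glue actor that, two seconds after BeginPlay, generates procedural glue geometry over meshes overlapping its Sphere using Geometry Script.
; It unions those meshes, builds a BVH, and projects seeded random points onto the nearest surface to append spheres.
; Morphological closing, smoothing and small-component removal fuse the spheres into one surface.
; SetupMesh, which would copy the result into the DynamicMeshComponent with its material, is not wired to run.
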(event Custom|AddGlue
  (Class|KismetMathLibrary|SeedRandomStream (Variables|Default|GetStream))
  (bind _components (CallFunction|GetOverlapComponent))
  (bind _dynamicmesh (CallFunction|CasttoDynamicComponent _components))
  (bind (_outputbvh _returnvalue) (Class|GeometryScriptLibraryMeshSpatial|BuildBVHforMesh _dynamicmesh 0))
  (bind _output_get (Variables|Default|SetBVH _outputbvh))
  (bind _output_get_2 (Variables|Default|SetDynamicMesh _returnvalue))
  (bind _outmesh (CallFunction|CalculateVertex _output_get _output_get_2))
  (bind _outmesh_2 (CallFunction|CalculateSurface _outmesh)))

(event EventBeginPlay
  (Utilities|FlowControl|Delay 2.0)
  (CallFunction|AddGlue)
  (Development|SetHiddeninGame (Variables|Default|GetSphere) true false))

(fn ConstructionScript)

(fn GetOverlapComponent
  (bind _outactors (Collision|ComponentOverlapActors (Variables|Default|GetSphere) (Transformation|GetWorldTransform (Variables|Default|GetSphere)) (Utilities|Array|MakeArray "ObjectTypeQuery1" "ObjectTypeQuery4" "ObjectTypeQuery2") 0 (Utilities|Array|MakeArray self)))
  (for _array_element _outactors
    (for _array_element_2 (Actor|GetComponentsByClass _array_element "/Script/Engine.MeshComponent")
      (Utilities|Array|AddUnique (LocalVariables|GetMeshComponentCache) _array_element_2)
      (Development|PrintString (Utilities|GetDisplayName _array_element_2) true true "(R=1.000000,G=0.967327,B=0.000000,A=1.000000)" 5.0)))
  (return (LocalVariables|GetMeshComponentCache)))

(fn CasttoDynamicComponent
  (params (Components :type Array%20of%20Mesh%20Component%20Object%20References))
  (LocalVariables|SetLocalComponents Components)
  (Utilities|FlowControl|Sequence
    (:then_0
      (bind _returnvalue (DynamicMeshActor|AllocateComputeMesh))
      (LocalVariables|SetDynamicMeshParent _returnvalue)
      (bind _returnvalue_2 (DynamicMeshActor|AllocateComputeMesh))
      (LocalVariables|SetDynamicMeshChild _returnvalue_2)
      (for _array_element (LocalVariables|GetLocalComponents)
        (GeometryScript|Scene|CopyMeshfromComponent :Component _array_element :ToDynamicMesh (LocalVariables|GetDynamicMeshChild) :bTransformToWorld true :Debug 0
          (:Success
            (GeometryScript|Booleans|ApplyMeshBoolean :TargetMesh (LocalVariables|GetDynamicMeshParent) :ToolMesh (LocalVariables|GetDynamicMeshChild) :Operation "Union" :Debug 0)
            (DynamicMesh|Reset (LocalVariables|GetDynamicMeshChild)))))
      (Class|GeometryScriptLibraryMeshRepairFunctions|CompactMesh (LocalVariables|GetDynamicMeshParent) 0))
    (:then_1
      (return (LocalVariables|GetDynamicMeshParent)))))

(fn CalculateVertex
  (params (BVH :type Geometry%20Script%20Dynamic%20Mesh%20BVH%20Structure) (DynamicMesh :type Dynamic%20Mesh%20Object%20Reference))
  (bind (_origin _boxextent) (Collision|GetActorBounds false false))
  (bind _stream (Variables|Default|GetStream))
  (LocalVariables|SetBVH_Local BVH)
  (LocalVariables|SetDynamicMeshLocal DynamicMesh)
  (bind _returnvalue (DynamicMeshActor|AllocateComputeMesh))
  (LocalVariables|SetVertexMesh _returnvalue)
  (Utilities|FlowControl|Sequence
    (:then_0
      (LocalVariables|SetOriginLocal _origin)
      (LocalVariables|SetBoxExtentLocal _boxextent)
      (for _index (range 0 (- (Variables|Default|GetDensity) 1))
        (bind _output_get (LocalVariables|SetQueryLocation (+ (LocalVariables|GetOriginLocal) (* (Math|Random|RandomFloatinRangefromStream _stream 0.0 (/ (+ (Class|KismetMathLibrary|GetMinElement (LocalVariables|GetBoxExtentLocal)) (Math|Vector|GetMaxElement (LocalVariables|GetBoxExtentLocal))) 2.0)) (Math|Random|RandomUnitVectorfromStream _stream)))))
        (bind (_nearestresult _returnvalue_2) (Class|GeometryScriptLibraryMeshSpatial|FindNearestPointonMesh :TargetMesh (LocalVariables|GetDynamicMeshLocal) :QueryBVH (LocalVariables|GetBVH_Local) :QueryPoint _output_get :Debug 0)
          (:Found
            (LocalVariables|SetPosition (.position _nearestresult))
            (LocalVariables|SetNormalVector (.ReturnValue (Class|GeometryScriptLibraryMeshQueryFunctions|GetTriangleFaceNormal _returnvalue_2 (.triangleid _nearestresult))))
            (if (.bIsValidTriangle (Class|GeometryScriptLibraryMeshQueryFunctions|GetTriangleFaceNormal _returnvalue_2 (.triangleid _nearestresult)))
              (Class|GeometryScriptLibraryMeshPrimitiveFunctions|AppendSphereBox (LocalVariables|GetVertexMesh) (Utilities|Struct|MakeGeometryScriptPrimitiveOptions "SingleGroup" false "Uniform") (Math|Transform|MakeTransform (+ (LocalVariables|GetPosition) (* (* (LocalVariables|GetNormalVector) (Variables|Default|GetThickness)) -0.7)) (Math|Rotator|MakeRotfromZ (LocalVariables|GetNormalVector)) "1.000000,1.000000,1.000000") (Variables|Default|GetThickness) 6 6 6 "Center" 0))))))
    (:then_1
      (return (LocalVariables|GetVertexMesh)))))

(fn SetupMesh
  (params (DynamicMesh :type Dynamic%20Mesh%20Object%20Reference))
  (bind _returnvalue (DynamicMeshComponent|GetDynamicMesh (Variables|DynamicMeshActor|GetDynamicMeshComponent)))
  (bind _output_get (LocalVariables|SetTargetMesh _returnvalue))
  (GeometryScript|MeshEdits|AppendMesh _output_get DynamicMesh (Math|Transform|InvertTransform (Transformation|GetActorTransform self)) false "(CombineMode=EnableAllMatching)" 0)
  (GeometryScript|Materials|EnableMaterialIDs (LocalVariables|GetTargetMesh) 0)
  (bind _returnvalue_2 (Class|DynamicMeshComponent|ValidateMaterialSlots (Variables|DynamicMeshActor|GetDynamicMeshComponent) true true))
  (if _returnvalue_2
    (Class|DynamicMeshComponent|ConfigureMaterialSet (Variables|DynamicMeshActor|GetDynamicMeshComponent) (Utilities|Array|MakeArray (Variables|Default|GetMaterial)))))

(fn CalculateSurface
  (params (DynamicMesh :type Dynamic%20Mesh%20Object%20Reference))
  (LocalVariables|SetLocalDynamicMesh DynamicMesh)
  (Utilities|FlowControl|Sequence
    (:then_0
      (Class|GeometryScriptLibraryMeshVoxelFunctions|ApplyMeshMorphology (LocalVariables|GetLocalDynamicMesh) (Utilities|Struct|MakeGeometryScriptMorphologyOptions (Utilities|Struct|MakeGeometryScript3DGridParameters "GridResolution" (Variables|Default|GetOptions%20SDFGrid%20Parameters%20Grid%20Cell%20Size) (Variables|Default|GetOptions%20SDFGrid%20Parameters%20Grid%20Resolution)) (Variables|Default|GetOptions%20Use%20Separate%20Mesh%20Grid) (Utilities|Struct|MakeGeometryScript3DGridParameters "GridResolution" (Variables|Default|GetOptions%20Mesh%20Grid%20Parameters%20Grid%20Cell%20Size) (Variables|Default|GetOptions%20Mesh%20Grid%20Parameters%20Grid%20Resolution)) "Close" (Variables|Default|GetOptions%20Distance)) 0)
      (Class|GeometryScriptLibraryMeshNormalsFunctions|ComputeTangents :TargetMesh (LocalVariables|GetLocalDynamicMesh) :Debug 0)
      (Class|GeometryScriptLibraryMeshNormalsFunctions|ComputeSplitNormals :TargetMesh (LocalVariables|GetLocalDynamicMesh) :SplitOptions (Utilities|Struct|MakeGeometryScriptSplitNormalsOptions true 9e+01 false "(bDefaultLayer=True,ExtendedLayerIndex=0)") :Debug 0))
    (:then_1
      (bind _returnvalue (Class|GeometryScriptLibraryMeshDeformFunctions|ApplyIterativeSmoothingtoMesh :TargetMesh (LocalVariables|GetLocalDynamicMesh) :Options (Utilities|Struct|MakeGeometryScriptIterativeMeshSmoothingOptions (Variables|Default|GetOptions%20Num%20Iterations) (Variables|Default|GetOptions%20Alpha) "FullMeshSelection") :Debug 0))
      (Class|GeometryScriptLibraryMeshRepairFunctions|RemoveSmallComponents _returnvalue (Utilities|Struct|MakeGeometryScriptRemoveSmallComponentOptions 0.0001 0.0001 (Variables|Default|GetOptions%20Min%20Triangle%20Count)) 0))
    (:then_2
      (return (LocalVariables|GetLocalDynamicMesh)))))