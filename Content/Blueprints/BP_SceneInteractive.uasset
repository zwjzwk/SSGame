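; BP_SceneInteractive is an interactive scene object whose physics-simulating meshes can switch to a pink or yellow MagGlow material and back.
; BeginPlay caches every material from those meshes in one flat InitialMaterials array.
; SetMaterialPink and SetMaterialYellow override all slots on the simulating meshes.
; SetMaterialOrigin restores the cache with a running index, relying on the same meshes simulating in the same order.
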(event Custom|SetMaterialPink
  (for _array_element (Actor|GetComponentsByClass "/Script/Engine.MeshComponent")
    (if (Physics|IsSimulatingPhysics _array_element "None")
      (for (_ _array_index) (Rendering|Material|GetMaterials _array_element)
        (Rendering|Material|SetMaterial _array_element _array_index "/Game/Assets/Materials/Magnesis/MI_MagGlowPink.MI_MagGlowPink")))))

(event Custom|SetMaterialOrigin
  (for _array_element (Actor|GetComponentsByClass "/Script/Engine.MeshComponent")
    (if (Physics|IsSimulatingPhysics _array_element "None")
      (for (_ _array_index) (Rendering|Material|GetMaterials _array_element)
        (Rendering|Material|SetMaterial _array_element _array_index (Utilities|Array|Get(acopy) (Variables|Default|GetInitialMaterials) (Variables|Default|GetMaterialIndex)))
        (Variables|Default|SetMaterialIndex (+ (Variables|Default|GetMaterialIndex) 1)))))
  (Variables|Default|SetMaterialIndex 0))

(event Custom|SetMaterialYellow
  (for _array_element (Actor|GetComponentsByClass "/Script/Engine.MeshComponent")
    (if (Physics|IsSimulatingPhysics _array_element "None")
      (for (_ _array_index) (Rendering|Material|GetMaterials _array_element)
        (Rendering|Material|SetMaterial _array_element _array_index "/Game/Assets/Materials/Magnesis/MI_MagGlowYellow.MI_MagGlowYellow")))))

(event EventBeginPlay
  (for _array_element (Actor|GetComponentsByClass "/Script/Engine.MeshComponent")
    (if (Physics|IsSimulatingPhysics _array_element "None")
      (for _array_element_2 (Rendering|Material|GetMaterials _array_element)
        (Utilities|Array|Add (Variables|Default|GetInitialMaterials) _array_element_2)))))

(fn ConstructionScript)