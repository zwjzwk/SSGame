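; BP_TipActor is a proximity trigger that shows an on-screen tip widget while the player is inside its sphere.
; When a BP_Player begins overlapping the Sphere, it creates a widget from the Widget class variable, stores it as CurrentWidget and adds it to the viewport.
; When the player's overlap ends, it removes the stored widget if valid, so each new entry builds a fresh one.
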(event OnComponentBeginOverlap(Sphere)
  (params (OverlappedComponent :type Primitive%20Component%20Object%20Reference) (OtherActor :type Actor%20Object%20Reference) (OtherComp :type Primitive%20Component%20Object%20Reference) (OtherBodyIndex :type Integer) (bFromSweep :type Boolean) (SweepResult :type Hit%20Result%20Structure%20%28by%20ref%29))
  (Utilities|Casting|CastToBP_Player OtherActor)
  (bind _returnvalue (UserInterface|CreateWidget (Variables|Default|GetWidget)))
  (bind _output_get (Variables|Default|SetCurrentWidget _returnvalue))
  (UserInterface|Viewport|AddtoViewport _output_get 0))

(event OnComponentEndOverlap(Sphere)
  (params (OverlappedComponent :type Primitive%20Component%20Object%20Reference) (OtherActor :type Actor%20Object%20Reference) (OtherComp :type Primitive%20Component%20Object%20Reference) (OtherBodyIndex :type Integer))
  (Utilities|Casting|CastToBP_Player OtherActor)
  (Utilities|IsValid (Variables|Default|GetCurrentWidget)
    (:Is%20Valid
      (Widget|RemovefromParent (Variables|Default|GetCurrentWidget)))))

(event EventBeginPlay)

(event Collision|EventActorBeginOverlap
  (params (OtherActor :type Actor%20Object%20Reference)))

(event EventTick
  (params (DeltaSeconds :type Float%20%28single-precision%29)))

(fn ConstructionScript)